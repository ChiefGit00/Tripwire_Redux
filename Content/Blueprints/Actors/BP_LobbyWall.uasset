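; BP_LobbyWall is a lobby wall actor that displays player details and a countdown through a WB_Lobby widget in its Widget component.
; On BeginPlay it casts and caches the widget.
; SetUpPlayer forwards a player's name and match record (played, won, lost) to the cached widget.
; StartTimer casts the component's widget again and calls its StartCountDown.
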(event Custom|SetUpPlayer
  (params (b :type Boolean) (PlayerName :type String) (MatchesPlayed :type String) (MatchesWon :type String) (MatchesLost :type String))
  (Default|SetPlayer (Variables|Default|GetWB_lobby) b PlayerName MatchesPlayed MatchesWon MatchesLost))

(event Custom|StartTimer
  (bind _aswb_lobby (Utilities|Casting|CastToWB_Lobby (UserInterface|GetUserWidgetObject (Variables|Default|GetWidget))))
  (Default|StartCountDown _aswb_lobby))

(event EventBeginPlay
  (bind _aswb_lobby (Utilities|Casting|CastToWB_Lobby (UserInterface|GetUserWidgetObject (Variables|Default|GetWidget))))
  (Variables|Default|SetWB_lobby _aswb_lobby))

(fn ConstructionScript)