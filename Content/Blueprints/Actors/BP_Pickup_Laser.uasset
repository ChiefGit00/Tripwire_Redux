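; Laser tripwire actor that alerts its owning player when another player character crosses its cylinder.
; A crossing notifies both players and restarts a looping timer that shows elapsed time since the breach on a widget.
; RenderT builds a render target and dynamic material from the laser's capture camera, fed to the owner's view for a brief delay.
; ShowAll and ShowOwnerOnly toggle whether only the owner sees the beam.
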(event OnComponentBeginOverlap(Cylinder)
  (params (OverlappedComponent :type Primitive%20Component%20Object%20Reference) (OtherActor :type Actor%20Object%20Reference) (OtherComp :type Primitive%20Component%20Object%20Reference) (OtherBodyIndex :type Integer) (bFromSweep :type Boolean) (SweepResult :type Hit%20Result%20Structure%20%28by%20ref%29))
  (bind _returnvalue (Components|GetOwner))
  (bind _returnvalue_2 (Transformation|GetActorLocation))
  ;[0.06667 0.06667 0.06667 0.2] Line Crossed
  (bind _asplayer_character (Utilities|Casting|CastToPlayerCharacter OtherActor))
  (if (not (== _asplayer_character _returnvalue))
    (Rendering|SetVisibility (Variables|Default|GetWidget) true false)
    (Default|LineCrossed _asplayer_character _returnvalue_2 false)
    (bind _asplayer_character_2 (Utilities|Casting|CastToPlayerCharacter _returnvalue))
    (Default|LineCrossed _asplayer_character_2 _returnvalue_2 true)
    (bind _returnvalue_3 (CallFunction|RenderT))
    (Default|LaserCamera _asplayer_character_2 true _returnvalue_3)
    (CallFunction|ResetOverlapTimer)
    (Variables|Default|SetTime 0.0)
    (bind _returnvalue_4 (Utilities|Time|SetTimerbyFunctionName 0 "OverlapLapsedTime" 0.5 true))
    (Utilities|FlowControl|Delay 2.0)
    (Default|LaserCamera _asplayer_character_2 false)))

(event Custom|OverlapLapsedTime
  ;[0.06667 0.06667 0.06667 0.2] Update Timer
  (bind _aswb_laser_timer (Utilities|Casting|CastToWB_LaserTimer (UserInterface|GetUserWidgetObject (Variables|Default|GetWidget))))
  (Default|UpdateTimer _aswb_laser_timer (Variables|Default|GetTime))
  (Variables|Default|SetTime (+ 0.5 (Variables|Default|GetTime))))

(event Custom|Reset%20Overlap%20Timer
  ;[0.06667 0.06667 0.06667 0.2] Line Crossed
  (Utilities|Time|ClearandInvalidateTimerbyHandle (stale OnComponentBeginOverlap(Cylinder) _returnvalue_4)))

(event EventShowAll
  (Rendering|SetOnlyOwnerSee (Variables|Default|GetCylinder) false :!class /Script/Engine.PrimitiveComponent))

(event EventShowOwnerOnly
  (Rendering|SetOnlyOwnerSee (Variables|Default|GetCylinder) true :!class /Script/Engine.PrimitiveComponent))

(fn ConstructionScript)

(fn RenderT
  (bind _lasercamera (Variables|Default|GetLaserCamera))
  (bind _returnvalue (Rendering|CreateRenderTarget2D 400 400 "RTF_RGBA16f"))
  (Variables|/Script/Engine.SceneCaptureComponent2D|SetTextureTarget _lasercamera _returnvalue)
  (bind _returnvalue_2 (Rendering|Material|CreateDynamicMaterialInstance "/Game/Materials/M_RenderTarget2D_Room01.M_RenderTarget2D_Room01" "None" :!class /Script/Engine.KismetMaterialLibrary))
  (Rendering|Material|SetTextureParameterValue _returnvalue_2 "ParamCapture" (Variables|/Script/Engine.SceneCaptureComponent2D|GetTextureTarget _lasercamera))
  (return _returnvalue_2))