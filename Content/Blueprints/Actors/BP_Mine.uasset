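; BP_Mine is a proximity mine that beeps every second and arms its trigger box one second after spawning.
; When a PlayerCharacter overlaps the box, it disables the trigger, deals full radial damage, hides its mesh, plays an explosion effect and sound, then destroys itself after a short delay.
; Separate events set the mesh visible to everyone, only to its owner, or to nobody.
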(event OnComponentBeginOverlap(Box)
  (params (OverlappedComponent :type Primitive%20Component%20Object%20Reference) (OtherActor :type Actor%20Object%20Reference) (OtherComp :type Primitive%20Component%20Object%20Reference) (OtherBodyIndex :type Integer) (bFromSweep :type Boolean) (SweepResult :type Hit%20Result%20Structure%20%28by%20ref%29))
  (Utilities|Casting|CastToPlayerCharacter OtherActor)
  (Collision|SetCollisionEnabled (Variables|Default|GetBox) "NoCollision")
  (Game|Damage|ApplyRadialDamage 5e+01 (Transformation|GetWorldLocation (Variables|Default|GetBox)) 2e+02 0 0 0 0 true "ECC_Visibility")
  (Rendering|SetVisibility (Variables|Default|GetCylinder) false false)
  (Effects|Components|ParticleSystem|SetTemplate (Variables|Default|GetParticleSystem) "/Game/Particles/Fire_Exp_02.Fire_Exp_02")
  (Audio|PlaySoundatLocation "/Game/Audio/Bomb+1.Bomb+1" (Transformation|GetActorLocation) "0, 0, 0" 1.0 1.0 0.0 0 0 0)
  (Utilities|FlowControl|Delay 1.5)
  (Actor|DestroyActor))

(event Custom|Beep
  (Audio|PlaySoundatLocation "/Game/Audio/Beep.Beep" (Transformation|GetWorldLocation (Variables|Default|GetDefaultSceneRoot)) "0, 0, 0" 6.0 1.0 0.0 "/Game/Audio/BeepAttenuation.BeepAttenuation" 0 0))

(event EventHideAll
  (Rendering|SetVisibility (Variables|Default|GetCylinder) false false))

(event EventShowAll
  (bind _cylinder (Variables|Default|GetCylinder))
  (Rendering|SetVisibility _cylinder true false)
  (Rendering|SetOnlyOwnerSee _cylinder false :!class /Script/Engine.PrimitiveComponent))

(event EventShowOwnerOnly
  (bind _cylinder (Variables|Default|GetCylinder))
  (Rendering|SetVisibility _cylinder true false)
  (Rendering|SetOnlyOwnerSee _cylinder true :!class /Script/Engine.PrimitiveComponent))

(event EventBeginPlay
  (Collision|SetCollisionEnabled (Variables|Default|GetBox) "NoCollision")
  (Utilities|Time|SetTimerbyFunctionName 0 "Beep" 1.0 true)
  (Utilities|FlowControl|Delay 1.0)
  (Collision|SetCollisionEnabled (Variables|Default|GetBox) "QueryAndPhysics"))

(fn ConstructionScript)