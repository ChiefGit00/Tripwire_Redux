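; Room actor with an on/off switch, a smoke effect and dropped tools.
; Its trigger registers the room with players; a nearby switch forwards clicks or touches through PC_Gameplay, and RoomSwitch toggles saved versus black materials and tool visibility.
; Smoke shows a wall for a timed period, hiding the stored player's health and looping coughs for others.
; ShowTrap briefly blacks out materials, raises the light and reveals all tools, then restores switch state.
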(event OnComponentBeginOverlap(Box)
  (params (OverlappedComponent :type Primitive%20Component%20Object%20Reference) (OtherActor :type Actor%20Object%20Reference) (OtherComp :type Primitive%20Component%20Object%20Reference) (OtherBodyIndex :type Integer) (bFromSweep :type Boolean) (SweepResult :type Hit%20Result%20Structure%20%28by%20ref%29))
  ;[1 1 1 1 24] Overlap Room
  (bind _asplayer_character (Utilities|Casting|CastToPlayerCharacter OtherActor))
  (Variables|/Game/Blueprints/Characters/PlayerCharacter.PlayerCharacter_C|SetbCan _asplayer_character true)
  (Variables|/Game/Blueprints/Characters/PlayerCharacter.PlayerCharacter_C|SetRoomRef _asplayer_character self)
  (if (Variables|Default|GetbSmoke)
    (if (== _asplayer_character (Variables|Default|GetPlayerChar))
      (Default|HideHealth (Variables|Default|GetPlayerChar) true)
      (else
        (Audio|PlaySoundatLocation "/Game/Audio/Cough.Cough" "0, 0, 0" "0, 0, 0" 1.0 1.0 0.0 0 0 0)
        (bind _returnvalue (Utilities|Time|SetTimerbyFunctionName 0 "PlayCough" 2.0 true))
        (Variables|Default|SetCoughTimer _returnvalue)))))

(event OnComponentEndOverlap(Box)
  (params (OverlappedComponent :type Primitive%20Component%20Object%20Reference) (OtherActor :type Actor%20Object%20Reference) (OtherComp :type Primitive%20Component%20Object%20Reference) (OtherBodyIndex :type Integer))
  (bind _playerchar (Variables|Default|GetPlayerChar))
  ;[1 1 1 1 24] Overlap Room
  (bind _asplayer_character (Utilities|Casting|CastToPlayerCharacter OtherActor))
  (Variables|/Game/Blueprints/Characters/PlayerCharacter.PlayerCharacter_C|SetbCan _asplayer_character false)
  (if (Variables|Default|GetbSmoke)
    (if (== _asplayer_character (Variables|Default|GetPlayerChar))
      (if (not (Pawn|IsLocallyControlled _playerchar))
        (Default|HideHealth _playerchar false))
      (else
        (Utilities|Time|ClearandInvalidateTimerbyHandle (Variables|Default|GetCoughTimer))))))

(event OnInputTouchBegin(W_Switch)
  (params (FingerIndex :type ETouchIndex%20Enum :default "Touch1") (TouchedComponent :type Primitive%20Component%20Object%20Reference))
  ;[1 1 1 1 24] Touch/Click Switch
  (if (Variables|Default|GetbAccess)
    (Rendering|SetVisibility (Variables|Default|GetW_SwitchHelp) false false)
    (bind _asplayer_character (Utilities|Casting|CastToPlayerCharacter (Game|Player|GetPlayerPawn 0)))
    (bind _output_get (Variables|Default|SetPlayerChar _asplayer_character))
    (Variables|/Game/Blueprints/Characters/PlayerCharacter.PlayerCharacter_C|SetbJump _output_get false)
    (bind _aspc_gameplay (Utilities|Casting|CastToPC_Gameplay (Game|GetPlayerController 0)))
    (Default|RoomSwitch _aspc_gameplay self)))

(event OnInputTouchEnd(W_Switch)
  (params (FingerIndex :type ETouchIndex%20Enum :default "Touch1") (TouchedComponent :type Primitive%20Component%20Object%20Reference))
  (bind _playerchar (Variables|Default|GetPlayerChar))
  ;[1 1 1 1 24] Touch/Click Switch
  (Utilities|IsValid _playerchar
    (:Is%20Valid
      (Variables|/Game/Blueprints/Characters/PlayerCharacter.PlayerCharacter_C|SetbJump _playerchar true))))

(event OnReleased(W_Switch)
  (params (TouchedComponent :type Primitive%20Component%20Object%20Reference) (ButtonReleased :type Key%20Structure))
  (bind _playerchar (Variables|Default|GetPlayerChar))
  ;[1 1 1 1 24] Touch/Click Switch
  (Utilities|IsValid _playerchar
    (:Is%20Valid
      (Variables|/Game/Blueprints/Characters/PlayerCharacter.PlayerCharacter_C|SetbJump _playerchar true))))

(event OnComponentBeginOverlap(b)
  (params (OverlappedComponent :type Primitive%20Component%20Object%20Reference) (OtherActor :type Actor%20Object%20Reference) (OtherComp :type Primitive%20Component%20Object%20Reference) (OtherBodyIndex :type Integer) (bFromSweep :type Boolean) (SweepResult :type Hit%20Result%20Structure%20%28by%20ref%29))
  ;[0.03646 0.03646 0.03646] Overlap Switch
  (Utilities|Casting|CastToPlayerCharacter OtherActor)
  (Rendering|Material|SetMaterial (Variables|Default|GetCube) 0 "/Game/Materials/M_SwitchActive.M_SwitchActive")
  (Variables|Default|SetbAccess true)
  (if (Variables|Default|GetbHelper)
    (Rendering|SetVisibility (Variables|Default|GetW_SwitchHelp) true false)))

(event OnClicked(W_Switch)
  (params (TouchedComponent :type Primitive%20Component%20Object%20Reference) (ButtonPressed :type Key%20Structure))
  ;[1 1 1 1 24] Touch/Click Switch
  (if (Variables|Default|GetbAccess)
    (Rendering|SetVisibility (Variables|Default|GetW_SwitchHelp) false false)
    (bind _asplayer_character (Utilities|Casting|CastToPlayerCharacter (Game|Player|GetPlayerPawn 0)))
    (bind _output_get (Variables|Default|SetPlayerChar _asplayer_character))
    (Variables|/Game/Blueprints/Characters/PlayerCharacter.PlayerCharacter_C|SetbJump _output_get false)
    (bind _aspc_gameplay (Utilities|Casting|CastToPC_Gameplay (Game|GetPlayerController 0)))
    (Default|RoomSwitch _aspc_gameplay self)))

(event OnComponentEndOverlap(b)
  (params (OverlappedComponent :type Primitive%20Component%20Object%20Reference) (OtherActor :type Actor%20Object%20Reference) (OtherComp :type Primitive%20Component%20Object%20Reference) (OtherBodyIndex :type Integer))
  ;[0.03646 0.03646 0.03646] Overlap Switch
  (Utilities|Casting|CastToPlayerCharacter OtherActor)
  (Rendering|Material|SetMaterial (Variables|Default|GetCube) 0 "/Game/Materials/M_SwitchDeactive.M_SwitchDeactive")
  (Variables|Default|SetbAccess false)
  (if (Variables|Default|GetbHelper)
    (Rendering|SetVisibility (Variables|Default|GetW_SwitchHelp) false false)))

(event Custom|ShowTrap
  ;[1 1 1] Show/Hide Trap
  (CallFunction|SetMaterial false)
  (Rendering|Components|Light|SetIntensity (Variables|Default|GetPointLight1) 2e+01)
  (for _array_element (Variables|Default|GetDroppedTools)
    (Utilities|IsValid _array_element
      (:Is%20Valid
        (bind _asbp_tool (Utilities|Casting|CastToBP_Tool _array_element))
        (Default|ShowAll _asbp_tool))))
  (Utilities|FlowControl|Delay 4.0)
  (CallFunction|HideTrap))

(event Custom|HideTrap
  ;[1 1 1] Show/Hide Trap
  (Rendering|Components|Light|SetIntensity (Variables|Default|GetPointLight1) 0.0)
  (if (Variables|Default|GetbSwitch)
    (CallFunction|SetMaterial true)
    (for _array_element (Variables|Default|GetDroppedTools)
      (Utilities|IsValid _array_element
        (:Is%20Valid
          (bind _asbp_tool (Utilities|Casting|CastToBP_Tool _array_element))
          (Default|ShowOwnerOnly _asbp_tool))))
    (else
      (CallFunction|SetMaterial false)
      (for _array_element_2 (Variables|Default|GetDroppedTools)
        (Utilities|IsValid _array_element_2
          (:Is%20Valid
            (bind _asbp_tool_2 (Utilities|Casting|CastToBP_Tool _array_element_2))
            (Default|HideAll _asbp_tool_2)))))))

(event Custom|SmokeOwner
  (params (Player :type Player%20Character%20Object%20Reference))
  ;[1 1 1 1 24] Smoke
  (Variables|Default|SetPlayerChar Player)
  (Variables|Default|SetbSmoke true)
  (Rendering|Material|SetMaterial (Variables|Default|GetSmokeWall) 0 "/Game/Materials/MI_SmokeLocal.MI_SmokeLocal"))

(event Custom|RoomSwitch
  (bind _droppedtools (Variables|Default|GetDroppedTools))
  ;[1 1 1 1 24] Room Switch
  (if (Variables|Default|GetbSwitch)
    (CallFunction|SetMaterial false)
    (Variables|Default|SetbSwitch false)
    (for _array_element _droppedtools
      (Utilities|IsValid _array_element
        (:Is%20Valid
          (bind _asbp_tool (Utilities|Casting|CastToBP_Tool _array_element))
          (Default|HideAll _asbp_tool))))
    (else
      (CallFunction|SetMaterial true)
      (Variables|Default|SetbSwitch true)
      (for _array_element_2 _droppedtools
        (Utilities|IsValid _array_element_2
          (:Is%20Valid
            (bind _asbp_tool_2 (Utilities|Casting|CastToBP_Tool _array_element_2))
            (Default|ShowOwnerOnly _asbp_tool_2)))))))

(event Custom|PlayCough
  (Audio|PlaySoundatLocation "/Game/Audio/Cough.Cough" "0, 0, 0" "0, 0, 0" 1.0 1.0 0.0 0 0 0))

(event Custom|ResetSmoke
  ;[1 1 1 1 24] Reset
  (Rendering|SetVisibility (Variables|Default|GetSmokeWall) false false)
  (Variables|Default|SetbSmoke false)
  (Utilities|Time|ClearandInvalidateTimerbyHandle (Variables|Default|GetCoughTimer)))

(event Custom|Smoke
  (params (PlayerChar :type Player%20Character%20Object%20Reference))
  (bind _smokewall (Variables|Default|GetSmokeWall))
  ;[1 1 1 1 24] Smoke
  (Variables|Default|SetPlayerChar PlayerChar)
  (Variables|Default|SetbSmoke true)
  (Rendering|SetVisibility _smokewall true false)
  (Rendering|Material|SetMaterial _smokewall 0 "/Game/Materials/MI_SmokeAll.MI_SmokeAll")
  (Utilities|FlowControl|Delay 3e+01)
  (Rendering|SetVisibility (Variables|Default|GetSmokeWall) false false)
  (Variables|Default|SetbSmoke false)
  (Utilities|Time|ClearandInvalidateTimerbyHandle (Variables|Default|GetCoughTimer)))

(event EventBeginPlay
  ;[1 1 1 1 24] Begin Play
  (CallFunction|SaveMaterials)
  (if (Variables|Default|GetbHelper)
    _))

(fn ConstructionScript)

(fn LightIntensity
  (params (InputPin :type Float%20%28single-precision%29))
  (Rendering|Components|Light|SetIntensity (Variables|Default|GetPointLight1) InputPin))

(fn LightColour
  (params (Condition :type Boolean))
  (bind _pointlight1 (Variables|Default|GetPointLight1))
  (if Condition
    (Rendering|Components|Light|SetLightColor _pointlight1 "(R=0.000000,G=1.000000,B=0.161544,A=1.000000)" true)
    (else
      (Rendering|Components|Light|SetLightColor _pointlight1 "(R=1.000000,G=1.000000,B=1.000000,A=1.000000)" true)))
  (return))

(fn CameraLocation
  (return (Transformation|GetWorldLocation (Variables|Default|GetSphere))))

(fn SetMaterial
  (params (b :type Boolean))
  (bind _staticmesh (Variables|Default|GetStaticMesh))
  (bind _staticmesh_2 (Variables|Default|GetStaticMesh))
  (bind _roommaterials (Variables|Default|GetRoomMaterials))
  (if b
    (Rendering|Material|SetMaterial _staticmesh 0 (Utilities|Array|Get(acopy) _roommaterials))
    (Rendering|Material|SetMaterial _staticmesh 1 (Utilities|Array|Get(acopy) _roommaterials 1))
    (Rendering|Material|SetMaterial _staticmesh 2 (Utilities|Array|Get(acopy) _roommaterials 2))
    (Rendering|Material|SetMaterial _staticmesh 3 (Utilities|Array|Get(acopy) _roommaterials 3))
    (Rendering|Material|SetMaterial _staticmesh 5 (Utilities|Array|Get(acopy) _roommaterials 5))
    (else
      (Rendering|Material|SetMaterial _staticmesh_2 0 "/Game/Materials/M_Black.M_Black")
      (Rendering|Material|SetMaterial _staticmesh_2 1 "/Game/Materials/M_Black.M_Black")
      (Rendering|Material|SetMaterial _staticmesh_2 2 "/Game/Materials/M_Black.M_Black")
      (Rendering|Material|SetMaterial _staticmesh_2 3 "/Game/Materials/M_Black.M_Black")
      (Rendering|Material|SetMaterial _staticmesh_2 5 "/Game/Materials/M_Black.M_Black"))))

(fn SaveMaterials
  (bind _staticmesh (Variables|Default|GetStaticMesh))
  (bind _roommaterials (Variables|Default|GetRoomMaterials))
  (Utilities|Array|Add _roommaterials (Rendering|Material|GetMaterial _staticmesh 0))
  (Utilities|Array|Add _roommaterials (Rendering|Material|GetMaterial _staticmesh 1))
  (Utilities|Array|Add _roommaterials (Rendering|Material|GetMaterial _staticmesh 2))
  (Utilities|Array|Add _roommaterials (Rendering|Material|GetMaterial _staticmesh 3))
  (Utilities|Array|Add _roommaterials (Rendering|Material|GetMaterial _staticmesh 5)))