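; GameInstanceTrip is a game instance that keeps the player's persistent name and game statistics.
; InitSaveGame loads the SaveGameTrip object from a single save slot, or creates one if none exists.
; Events update the name and played, won and lost counts, or reset them, writing to disk immediately, while getters expose those values.
; A running game time total accumulates on the instance itself and is not written to the save.
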(event Custom|InitSaveGame
  (bind _returnvalue (SaveGame|DoesSaveGameExist "save"))
  (if _returnvalue
    (bind _returnvalue_2 (SaveGame|LoadGamefromSlot "save"))
    (bind _assave_game_trip (Utilities|Casting|CastToSaveGameTrip _returnvalue_2))
    (Variables|Default|SetSaveGame _assave_game_trip)
    (else
      (bind _returnvalue_3 (SaveGame|CreateSaveGameObject "/Game/Blueprints/AllLevels/SaveGameTrip.SaveGameTrip_C"))
      (Variables|Default|SetSaveGame _returnvalue_3))))

(event Custom|IncSaveGamesPlayed
  (bind _savegame (Variables|Default|GetSaveGame))
  (bind _result (Math|Integer|IncrementInt (Variables|/Game/Blueprints/AllLevels/SaveGameTrip.SaveGameTrip_C|GetGamesPlayed _savegame))
    (:%20%20
      (Variables|/Game/Blueprints/AllLevels/SaveGameTrip.SaveGameTrip_C|SetGamesPlayed _savegame _result)
      (SaveGame|SaveGametoSlot _savegame "save"))))

(event Custom|SaveGamesLost
  (bind _savegame (Variables|Default|GetSaveGame))
  (bind _result (Math|Integer|IncrementInt (Variables|/Game/Blueprints/AllLevels/SaveGameTrip.SaveGameTrip_C|GetGamesLost _savegame))
    (:%20%20
      (Variables|/Game/Blueprints/AllLevels/SaveGameTrip.SaveGameTrip_C|SetGamesLost _savegame _result)
      (SaveGame|SaveGametoSlot _savegame "save"))))

(event Custom|SaveGamesWon
  (bind _savegame (Variables|Default|GetSaveGame))
  (bind _result (Math|Integer|IncrementInt (Variables|/Game/Blueprints/AllLevels/SaveGameTrip.SaveGameTrip_C|GetGamesWon _savegame))
    (:%20%20
      (Variables|/Game/Blueprints/AllLevels/SaveGameTrip.SaveGameTrip_C|SetGamesWon _savegame _result)
      (SaveGame|SaveGametoSlot _savegame "save"))))

(event Custom|ResetSaveGame
  (bind _savegame (Variables|Default|GetSaveGame))
  (Variables|/Game/Blueprints/AllLevels/SaveGameTrip.SaveGameTrip_C|SetPlayerName _savegame "")
  (Variables|/Game/Blueprints/AllLevels/SaveGameTrip.SaveGameTrip_C|SetGamesPlayed _savegame 0)
  (Variables|/Game/Blueprints/AllLevels/SaveGameTrip.SaveGameTrip_C|SetGamesWon _savegame 0)
  (Variables|/Game/Blueprints/AllLevels/SaveGameTrip.SaveGameTrip_C|SetGamesLost _savegame 0)
  (Variables|/Game/Blueprints/AllLevels/SaveGameTrip.SaveGameTrip_C|SetGamesQuit _savegame 0)
  (SaveGame|SaveGametoSlot _savegame "save")
  (Development|PrintString "Reset"))

(event Custom|SavePlayerName
  (params (PlayerName :type String))
  (bind _savegame (Variables|Default|GetSaveGame))
  (Variables|/Game/Blueprints/AllLevels/SaveGameTrip.SaveGameTrip_C|SetPlayerName _savegame PlayerName)
  (SaveGame|SaveGametoSlot _savegame "save"))

(fn AddGameTime
  (params (GameTimeAdd :type Integer))
  (Variables|Default|SetGameTime (+ GameTimeAdd (Variables|Default|GetGameTime))))

(fn GetTotalGameTime
  (return (Variables|Default|GetGameTime)))

(fn GetPlayerName
  (return (Variables|/Game/Blueprints/AllLevels/SaveGameTrip.SaveGameTrip_C|GetPlayerName (Variables|Default|GetSaveGame))))

(fn GetGamesPlayed
  (return (Variables|/Game/Blueprints/AllLevels/SaveGameTrip.SaveGameTrip_C|GetGamesPlayed (Variables|Default|GetSaveGame))))

(fn GetGamesWon
  (return (Variables|/Game/Blueprints/AllLevels/SaveGameTrip.SaveGameTrip_C|GetGamesWon (Variables|Default|GetSaveGame))))

(fn GetGamesLost
  (return (Variables|/Game/Blueprints/AllLevels/SaveGameTrip.SaveGameTrip_C|GetGamesLost (Variables|Default|GetSaveGame))))