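; Lobby player controller that loads the player's name and match record and shows them on the lobby wall.
; Initialize reads the save through GameInstanceTrip, then after a short delay passes the data to a server player-data event and to BP_LobbyWall.
; A countdown event starts the wall's timer after a brief delay.
; BeginPlay activates the virtual joystick touch interface and adds the lobby HUD.
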(event Custom|S_PlayerData
  (params (PlayerName :type String) (GamesWon :type String) (GamesLost :type String) (GamesPlayed :type String))
  ;[1 1 1] Server Player Data
  (Variables|Default|SetPlayerName PlayerName)
  (Variables|Default|SetGamesWon GamesWon)
  (Variables|Default|SetGamesLost GamesLost)
  (Variables|Default|SetGamesPlayed GamesPlayed))

(event Custom|Initialize
  ;[1 1 1] Initialize
  (Variables|Default|SetbShowMouseCursor true)
  (bind _asgame_instance_trip (Utilities|Casting|CastToGameInstanceTrip (Game|GetGameInstance)))
  (bind _output_get (Variables|Default|SetSaveGame _asgame_instance_trip))
  (Default|InitSaveGame _output_get)
  (Variables|Default|SetPlayerName (Default|GetPlayerName (Variables|Default|GetSaveGame)))
  (Variables|Default|SetGamesWon (Utilities|String|ToString(Integer) (Default|GetGamesWon (Variables|Default|GetSaveGame))))
  (Variables|Default|SetGamesLost (Utilities|String|ToString(Integer) (Default|GetGamesLost (Variables|Default|GetSaveGame))))
  (Variables|Default|SetGamesPlayed (Utilities|String|ToString(Integer) (Default|GetGamesPlayed (Variables|Default|GetSaveGame))))
  (Utilities|FlowControl|Delay 0.5)
  (CallFunction|SPlayerData (Variables|Default|GetPlayerName) (Variables|Default|GetGamesWon) (Variables|Default|GetGamesLost) (Variables|Default|GetGamesPlayed))
  (CallFunction|SetUpPlayer true (Variables|Default|GetPlayerName) (Variables|Default|GetGamesPlayed) (Variables|Default|GetGamesWon) (Variables|Default|GetGamesLost)))

(event Custom|SetUpPlayer
  (params (b :type Boolean) (PlayerName :type String) (MatchesPlayed :type String) (MatchesWon :type String) (MatchesLost :type String))
  ;[1 1 1] SetUp Player/Enemy
  (bind _returnvalue (Actor|GetActorOfClass "/Game/Blueprints/Actors/BP_LobbyWall.BP_LobbyWall_C"))
  (Default|SetUpPlayer _returnvalue b PlayerName MatchesPlayed MatchesWon MatchesLost))

(event Custom|StartCountdown
  ;[1 1 1] Count Down Timer
  (Utilities|FlowControl|Delay 0.2)
  (bind _returnvalue (Actor|GetActorOfClass "/Game/Blueprints/Actors/BP_LobbyWall.BP_LobbyWall_C"))
  (Default|StartTimer _returnvalue))

(event EventBeginPlay
  ;[1 1 1] Activate Touch
  (Class|PlayerController|ActivateTouchInterface "/Game/Blueprints/AllLevels/LeftVirtualJoystick.LeftVirtualJoystick")
  (bind _returnvalue (UserInterface|CreateWidget "/Game/UI/WB_LobbyHUD.WB_LobbyHUD_C"))
  (UserInterface|Viewport|AddtoViewport _returnvalue 0))

(fn ConstructionScript)