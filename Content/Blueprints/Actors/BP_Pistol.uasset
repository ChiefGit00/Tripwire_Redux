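; BP_Pistol is a single-shot pistol actor that damages a player character and is then reported as used.
; Fire waits briefly, plays the shot sound and runs a short visibility trace offset only along world X by the owner's forward X component.
; A PlayerCharacter hit takes fixed damage.
; After further delays the mesh visibility toggles, and the authority calls OCWeaponUsed on the owning character.
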(event Custom|Fire
  (bind _defaultsceneroot (Variables|Default|GetDefaultSceneRoot))
  (bind _returnvalue (Transformation|GetWorldLocation _defaultsceneroot))
  ;[0.06667 0.06667 0.06667 0.2] Fire
  (Utilities|FlowControl|Delay 0.4)
  (Audio|PlaySoundatLocation "/Game/Audio/Barreta.Barreta" _returnvalue "0, 0, 0" 1.0 1.0 0.0 0 0 0)
  (bind _outhit (Collision|LineTraceByChannel _returnvalue (+ _returnvalue (Math|Vector|MakeVector (* (.x (Transformation|GetActorForwardVector (Components|GetOwner))) 5.5e+02) 0.0 0.0)) "TraceTypeQuery1" false 0 "None"))
  (bind _asplayer_character (Utilities|Casting|CastToPlayerCharacter (.hitactor _outhit))
    (:then
      (Game|Damage|ApplyDamage _asplayer_character 5e+01 0 0))
    (:CastFailed
      _))
  (Utilities|FlowControl|Delay 0.4)
  (Rendering|ToggleVisibility (Variables|Default|GetSkeletalMesh) false)
  (Utilities|FlowControl|Delay 0.3)
  (Networking|SwitchHasAuthority
    (:Authority
      (bind _asplayer_character_2 (Utilities|Casting|CastToPlayerCharacter (Components|GetOwner)))
      (Default|OCWeaponUsed _asplayer_character_2 "Pistol"))))

(fn ConstructionScript)