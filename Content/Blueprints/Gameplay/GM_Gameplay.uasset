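; Gameplay game mode that runs a round-based match between player controllers and tracks who lost each round.
; MatchOver updates scores, then either resets the round by clearing tools, weapons and smoke and respawning characters at PlayerStarts, or ends the game.
; GameQuit forfeits the match for the quitting player; both endings notify controllers, then open the Lobby after a delay.
; PlayersCtrls registers each controller and returns its spawn transform.
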(event Custom|GameOver
  ;[0.06667 0.06667 0.06667 0.2] Match Over
  (Development|ExecuteConsoleCommand "open  Lobby" 0))

(event Custom|GameQuit
  (params (PlayerLost :type PC%20Gameplay%20Object%20Reference))
  ;[0.06667 0.06667 0.06667 0.2] Match Over
  (Variables|Default|SetPlayerLost PlayerLost)
  (for _array_element (Variables|Default|GetPlayerCtrls)
    (if (== (Variables|Default|GetPlayerLost) _array_element)
      (Variables|/Game/Blueprints/Gameplay/PC_Gameplay.PC_Gameplay_C|SetEnemyScore _array_element 2)
      (else
        (Variables|/Game/Blueprints/Gameplay/PC_Gameplay.PC_Gameplay_C|SetScore _array_element 2))))
  (Utilities|FlowControl|Delay 1.0)
  (for _array_element_2 (Variables|Default|GetPlayerCtrls)
    (Default|GameOver _array_element_2))
  (Utilities|FlowControl|Delay 3.0)
  (CallFunction|GameOver))

(event Custom|MatchOver
  (params (PlayerLost :type PC%20Gameplay%20Object%20Reference))
  ;[0.06667 0.06667 0.06667 0.2] Match Over
  (Variables|Default|SetPlayerLost PlayerLost)
  (for _array_element (Variables|Default|GetPlayerCtrls)
    (if (== (Variables|Default|GetPlayerLost) _array_element)
      (bind _result (Math|Integer|IncrementInt (Variables|/Game/Blueprints/Gameplay/PC_Gameplay.PC_Gameplay_C|GetEnemyScore _array_element))
        (:%20%20
          (if (> _result 1)
            (Variables|Default|SetbGameOver true))))
      (else
        (bind _result_2 (Math|Integer|IncrementInt (Variables|/Game/Blueprints/Gameplay/PC_Gameplay.PC_Gameplay_C|GetScore _array_element))
          (:%20%20
            (if (> _result_2 1)
              (Variables|Default|SetbGameOver true)))))))
  (if (Variables|Default|GetbGameOver)
    (for _array_element_2 (Variables|Default|GetPlayerCtrls)
      (Default|GameOver _array_element_2))
    (Utilities|FlowControl|Delay 3.0)
    (CallFunction|GameOver)
    (else
      (bind _outactors (Actor|GetAllActorsOfClass "/Game/Blueprints/Actors/BP_Tool.BP_Tool_C"))
      (for _array_element_3 _outactors
        (Actor|DestroyActor _array_element_3))
      (bind _outactors_2 (Actor|GetAllActorsOfClass "/Game/Blueprints/Actors/BP_Weapon.BP_Weapon_C"))
      (for _array_element_4 _outactors_2
        (Actor|DestroyActor _array_element_4))
      (bind _outactors_3 (Actor|GetAllActorsOfClass "/Game/Blueprints/Actors/BP_Room.BP_Room_C"))
      (for _array_element_5 _outactors_3
        (Default|ResetSmoke _array_element_5))
      (for (_array_element_6 _array_index) (Variables|Default|GetPlayerCtrls)
        (Utilities|IsValid (Pawn|GetControlledPawn _array_element_6)
          (:Is%20Valid
            (Actor|DestroyActor (Pawn|GetControlledPawn _array_element_6)))
          (:Is%20Not%20Valid
            _))
        (bind _returnvalue (Game|SpawnActorfromClass "/Game/Blueprints/Characters/PlayerCharacter.PlayerCharacter_C" (Transformation|GetActorTransform (Utilities|Array|Get(acopy) (Variables|Default|GetSpawnPoints) _array_index)) "Undefined" 0 0))
        (Default|Reset _array_element_6)
        (Pawn|Possess _array_element_6 _returnvalue)))))

(event EventBeginPlay
  ;[0.06667 0.06667 0.06667 0.2] Get Player Controllers
  (bind _outactors (Actor|GetAllActorsOfClass "/Script/Engine.PlayerStart"))
  (Variables|Default|SetSpawnPoints _outactors))

(fn ConstructionScript)

(fn PlayersCtrls
  (params (Ctrl :type PC%20Gameplay%20Object%20Reference%20%28by%20ref%29))
  (bind _returnvalue (Utilities|Array|Add (Variables|Default|GetPlayerCtrls) Ctrl))
  (return (Transformation|GetActorTransform (Utilities|Array|Get(acopy) (Variables|Default|GetSpawnPoints) _returnvalue))))