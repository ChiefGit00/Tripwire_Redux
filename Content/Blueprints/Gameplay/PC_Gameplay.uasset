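; Player controller for a networked match game with scores against an enemy player, handling possession, HUD, sessions and match results.
; On authority BeginPlay it spawns and possesses a PlayerCharacter and loads save data from the game instance.
; A DataTable-built inventory feeds dropped devices, weapons, vision tools and timer-drained Stealth/Sprint abilities, consuming items by hard-coded index.
; Server events handle spawning and attacks, while RepNotify health and scores update the HUD.
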(event Custom|Drop
  (params (DeviceName :type String))
  (bind _playerchar (Variables|Default|GetPlayerChar))
  (bind _returnvalue (Transformation|GetActorLocation _playerchar))
  ;[0.06667 0.06667 0.06667 0.06667] Use Drop Devices
  (if (Variables|/Game/Blueprints/Characters/PlayerCharacter.PlayerCharacter_C|GetbCan (Variables|Default|GetPlayerChar))
    (bind (_actorclass _transform) (CallFunction|InventoryDrop DeviceName))
    (bind _outactors (Actor|GetAllActorsOfClass "/Game/Blueprints/Characters/PlayerCharacter.PlayerCharacter_C"))
    (bind _outhit (Collision|LineTraceByChannel (+ _returnvalue "20.000000, 0,-10.000000") (+ _returnvalue "0, 0,-400.000000") "TraceTypeQuery2" false _outactors "None"))
    (Utilities|FlowControl|Delay 0.0)
    (CallFunction|SSpawnDevice _actorclass (Math|Transform|MakeTransform (+ (.location _outhit) _transform)))
    (Default|CallCallHUDRefresh)
    (Utilities|FlowControl|Delay 0.2)
    (if (Utilities|Enum|Equal(Enum) "Camera" DeviceName)
      (CallFunction|PawnCameraSetup))))

(event Custom|RoomSmoke
  (bind _playerchar (Variables|Default|GetPlayerChar))
  ;[0.06667 0.06667 0.06667 0.06667] Server Room Smoke
  (Default|Smoke (Variables|/Game/Blueprints/Characters/PlayerCharacter.PlayerCharacter_C|GetRoomRef _playerchar) _playerchar)
  (CallFunction|RoomSmokeOwner))

(event Custom|UseVision
  (params (VisionName :type String))
  (bind _playerchar (Variables|Default|GetPlayerChar))
  (bind _hud (Variables|Default|GetHUD))
  ;[0.06667 0.06667 0.06667 0.06667] Use Vision
  (Default|ToolsHide (Variables|Default|GetHUD) false)
  (Default|SetScope (Variables|Default|GetPlayerChar) false)
  (switch string VisionName
    (:Scope
      (CallFunction|InventoryConsume 4 1)
      (if (Variables|Default|GetbScope)
        (Default|F11 _hud true)
        (Default|SetScope _playerchar true)
        (Variables|Default|SetbScope false)
        (Utilities|FlowControl|Delay 3.0))
      (Default|F11 _hud false)
      (Default|SetScope _playerchar false)
      (Variables|Default|SetbScope true)
      (Default|PickUpRefresh (Variables|Default|GetHUD) "NewEnumerator1"))
    (:Traps
      (CallFunction|InventoryConsume 3 1)
      (Default|ShowTrap (Variables|/Game/Blueprints/Characters/PlayerCharacter.PlayerCharacter_C|GetRoomRef (Variables|Default|GetPlayerChar)))
      (Default|PickUpRefresh (Variables|Default|GetHUD) "NewEnumerator1"))))

(event Custom|Join
  ;[0.06667 0.06667 0.06667 0.06667] Host/Join
  (bind _results (|FindSessions self 2 false)
    (:OnSuccess
      (|JoinSession self (Utilities|Array|Get(acopy) _results)
        (:OnFailure
          (Development|PrintString (Utilities|String|ToString(Integer) (Utilities|Array|Length _results))))))
    (:OnFailure
      (Development|PrintString "Failed to join")
      (Default|StopLANHostJoin (Variables|Default|GetWBLevels)))))

(event Custom|UseAbility
  (params (bActivate :type Boolean) (Name :type String))
  ;[0.06667 0.06667 0.06667 0.06667] Expend Abilities
  ;;[1 1 1] UseAbility
  (CallFunction|ActivateAbility bActivate Name))

(event Custom|GetPickUp
  (params (PickUpName :type String) (Count :type Integer))
  ;[0.06667 0.06667 0.06667 0.06667] Get Inventory
  (bind (_array_element _array_index) (Utilities|Array|ForEachLoopwithBreak (Variables|Default|GetInventory) :!label _label)
    (:LoopBody
      (if (Utilities|Enum|Equal(Enum) PickUpName (.itemname _array_element))
        (if (>= (.maxcount _array_element) (+ (.count _array_element) Count))
          (Utilities|Array|SetArrayElem (Variables|Default|GetInventory) _array_index (Utilities|Struct|MakePickUps (.itemtype _array_element) (.itemname _array_element) (.itemdescription _array_element) (.itemicon _array_element) (+ (.count _array_element) Count) (.maxcount _array_element) (.probability _array_element)))
          (goto _label Break))))
    (:Completed
      (CallFunction|RefreshHUD)
      (CallFunction|UseAbility false))))

(event Custom|ExpendAbility
  (bind _playerchar (Variables|Default|GetPlayerChar))
  (bind _returnvalue (Transformation|GetVelocity _playerchar))
  (bind _returnvalue_2 (Math|Vector|VectorLength _returnvalue))
  (bind _returnvalue_3 (> _returnvalue_2 0.0))
  ;[0.06667 0.06667 0.06667 0.06667] Expend Abilities
  (switch string (Variables|Default|GetActiveAbilityName)
    (:Stealth
      (if _returnvalue_3
        (Variables|Default|SetcurStealth (- (Variables|Default|GetcurStealth) 0.04))
        (else
          (Variables|Default|SetcurStealth (- (Variables|Default|GetcurStealth) 0.04))))
      (if (<= (Variables|Default|GetcurStealth) 0.0)
        (CallFunction|InventoryConsume 6 1)
        (Variables|Default|SetcurStealth 1.0)
        (Default|PickUpRefresh (Variables|Default|GetHUD) "NewEnumerator2")
        (CallFunction|UseAbility false :!label _label)
        (else
          (Default|CallDAbilityCurrentValue (Variables|Default|GetcurStealth)))))
    (:Sprint
      (if _returnvalue_3
        (if (not (Variables|/Game/Blueprints/Characters/PlayerCharacter.PlayerCharacter_C|GetbCrouch (Variables|Default|GetPlayerChar)))
          (bind _output_get (Variables|Default|SetcurSprint (- (Variables|Default|GetcurSprint) 0.08)))
          (if (<= _output_get 0.0)
            (CallFunction|InventoryConsume 8 1)
            (Variables|Default|SetcurSprint 1.0)
            (Default|PickUpRefresh (Variables|Default|GetHUD) "NewEnumerator2")
            (goto _label)
            (else
              (Default|CallDAbilityCurrentValue _output_get))))))))

(event Custom|Attack
  (params (bPunch :type Boolean) (AttackName :type String))
  ;[0.06667 0.06667 0.06667 0.06667] Melee Attack
  (if bPunch
    (switch string AttackName
      (:Sword
        (CallFunction|SCharAttack bPunch AttackName :!label _label))
      (:Pistol
        (bind _bconsumed (CallFunction|InventoryConsume 12 1))
        (if _bconsumed
          (goto _label)))
      (:Bomb
        (bind _bconsumed_2 (CallFunction|InventoryConsume 13 1))
        (if _bconsumed_2
          (goto _label))))
    (else
      (goto _label))))

(event Custom|HUDPickUPHide
  (params (bNow :type Boolean))
  ;[1 1 1] PickUp HUD
  (Default|HidePickUps (Variables|Default|GetHUD))
  (CallFunction|ClosPickUp bNow))

(event Custom|HUDPickUPShow
  (params (PickUps :type Array%20of%20Pick%20Ups%20Counts%20Structures))
  ;[1 1 1] PickUp HUD
  (Default|DisplayPickUps (Variables|Default|GetHUD) PickUps))

(event Custom|RoomSmokeOwner
  (bind _playerchar (Variables|Default|GetPlayerChar))
  ;[0.06667 0.06667 0.06667 0.06667] Server Room Smoke
  (Default|SmokeOwner (Variables|/Game/Blueprints/Characters/PlayerCharacter.PlayerCharacter_C|GetRoomRef _playerchar) _playerchar))

(event Custom|S_UseWeapon
  (params (Weapon :type String))
  ;[0.06667 0.06667 0.06667 0.06667] Use Weapon
  (CallFunction|OCUseWeapon Weapon))

(event Custom|PickUpAnim
  (params (PickUp :type BP%20Pick%20Up%20Object%20Reference) (bOpen :type Boolean) (bNow :type Boolean))
  ;[0.06667 0.06667 0.06667 0.06667] Get Pick Up Animation
  (bind _output_get (Variables|Default|SetPickUpRef PickUp))
  (if bNow
    (Default|PlayOpenAnimation _output_get bOpen 0.6)
    (else
      (Default|PlayOpenAnimation _output_get bOpen (Math|Conversions|ToFloat(Integer) (Math|Random|RandomIntegerinRange 5 15))))))

(event Custom|OC_UseWeapon
  (params (Weapon :type String))
  ;[0.06667 0.06667 0.06667 0.06667] Use Weapon
  (switch string Weapon
    (:Sword
      (CallFunction|InventoryConsume 2 1)
      (CallFunction|SEquipWeapon))
    (:Pistol
      (CallFunction|SEquipWeapon :!label _label))
    (:Bomb
      (goto _label)))
  (Default|PickUpRefresh (Variables|Default|GetHUD) "NewEnumerator0"))

(event Custom|MatchOver
  ;[0.06667 0.06667 0.06667 0.06667] Match/Game Over
  (bind _asgm_gameplay (Utilities|Casting|CastToGM_Gameplay (Game|GetGameMode)))
  (Default|MatchOver _asgm_gameplay self))

(event Custom|MatchPrep
  ;[0.06667 0.06667 0.06667 0.06667] Match/Game Over
  (Utilities|FlowControl|Delay 3.0)
  (CallFunction|MatchOver))

(event Custom|Reset
  ;[0.06667 0.06667 0.06667 0.06667] Inventory Reset
  (CallFunction|InventoryReset)
  (Variables|Default|SetHealth 1e+02)
  (Variables|Default|SetcurStealth 1.0)
  (Variables|Default|SetcurSprint 1.0)
  (Utilities|Time|ClearTimerbyFunctionName 0 "ExpendAbility"))

(event Custom|S_PCtrlName
  (params (PlayerName :type String))
  ;[0.06667 0.06667 0.06667 0.06667] Player Char Name
  (Variables|Default|SetName PlayerName))

(event Custom|QuitGame
  ;[0.06667 0.06667 0.06667 0.06667] Match/Game Over
  (bind _asgm_gameplay (Utilities|Casting|CastToGM_Gameplay (Game|GetGameMode)))
  (Default|GameQuit _asgm_gameplay self))

(event Custom|GameOver
  (bind _savegameinstance (Variables|Default|GetSaveGameInstance))
  (bind _enemyscore (Variables|Default|GetEnemyScore))
  ;[0.06667 0.06667 0.06667 0.06667] Game Over
  (Viewport|RemoveAllWidgets)
  (bind _returnvalue (UserInterface|CreateWidget "/Game/UI/WB_MatchOver.WB_MatchOver_C"))
  (UserInterface|Viewport|AddtoViewport _returnvalue 0)
  (Development|PrintString (Utilities|String|ToString(Integer) _enemyscore))
  (if (> (Variables|Default|GetScore) _enemyscore)
    (Default|SaveGamesWon _savegameinstance)
    (Default|GameOver _returnvalue "Winner")
    (Audio|SpawnSound2D "/Game/Audio/Small_Croud_Applause_2.Small_Croud_Applause_2" 1.0 1.0 0.0 0)
    (else
      (Default|SaveGamesLost _savegameinstance)
      (Default|GameOver _returnvalue "Lost")
      (Audio|SpawnSound2D "/Game/Audio/awww.awww" 1.0 1.0 0.0 0))))

(event Custom|LaserCameraSetup
  (params (b :type Boolean) (Material :type Material%20Interface%20Object%20Reference))
  ;[0.06667 0.06667 0.06667 0.06667] Laser Camera
  (Class|Image|SetBrushfromMaterial (Variables|/Game/UI/WB_HUD.WB_HUD_C|GetImage_LaserCamera (Variables|Default|GetHUD)) Material)
  (Default|LaserCamera (Variables|Default|GetHUD) b))

(event Custom|S_CharAttack
  (params (bPunch :type Boolean) (AttackName :type String))
  ;[0.06667 0.06667 0.06667 0.06667] Melee Attack
  (Default|CharAttack (Variables|Default|GetPlayerChar) bPunch AttackName))

(event Custom|PlayerCharName
  (params (PlayerName :type String))
  ;[0.06667 0.06667 0.06667 0.06667] Player Char Name
  (Variables|/Game/Blueprints/Characters/PlayerCharacter.PlayerCharacter_C|SetPlayerName (Variables|Default|GetPlayerChar) PlayerName))

(event Custom|UpdateScore
  (params (Condition :type Boolean) (Score :type Integer))
  (bind _returnvalue (Utilities|Text|ToText(Integer) Score))
  ;[0.06667 0.06667 0.06667 0.06667] UpdateScore
  (if Condition
    (Rendering|Components|TextRender|SetText (Variables|/Game/UI/WB_HUD.WB_HUD_C|GetText_PlayerScore (Variables|Default|GetHUD)) _returnvalue)
    (else
      (Rendering|Components|TextRender|SetText (Variables|/Game/UI/WB_HUD.WB_HUD_C|GetText_EnemyScore (Variables|Default|GetHUD)) _returnvalue))))

(event Custom|GameOverUI
  (bind _self self)
  ;[0.06667 0.06667 0.06667 0.06667] Game Over UI
  (Viewport|RemoveAllWidgets)
  (Variables|Default|SetbShowMouseCursor _self true)
  (Variables|Default|SetbEnableMouseOverEvents _self true)
  (bind _returnvalue (UserInterface|CreateWidget "/Game/UI/WB_MatchOver.WB_MatchOver_C"))
  (UserInterface|Viewport|AddtoViewport _returnvalue 0))

(event Custom|SetUp
  ;[0.06667 0.06667 0.06667 0.06667] Begin Play (SaveGameInstance, GameMode send PCtrl)
  (bind _asgame_instance_trip (Utilities|Casting|CastToGameInstanceTrip (Game|GetGameInstance)))
  (bind _output_get (Variables|Default|SetSaveGameInstance _asgame_instance_trip))
  (Default|InitSaveGame _output_get)
  (Default|IncSaveGamesPlayed (Variables|Default|GetSaveGameInstance))
  (CallFunction|SPCtrlName (Default|GetPlayerName (Variables|Default|GetSaveGameInstance))))

(event Custom|UpdatePlayerName
  (params (Condition :type Boolean) (Name :type String))
  (bind _returnvalue (Utilities|Text|ToText(String) Name))
  ;[0.06667 0.06667 0.06667 0.06667] Player/Enemy Name
  (if Condition
    (Rendering|Components|TextRender|SetText (Variables|/Game/UI/WB_HUD.WB_HUD_C|GetText_PlayerName (Variables|Default|GetHUD)) _returnvalue)
    (else
      (Rendering|Components|TextRender|SetText (Variables|/Game/UI/WB_HUD.WB_HUD_C|GetText_EnemyName_1 (Variables|Default|GetHUD)) _returnvalue))))

(event Custom|RoomSwitch
  (params (RoomRef :type BP%20Room%20Object%20Reference))
  ;[0.06667 0.06667 0.06667 0.06667] Room Switch
  (Default|RoomSwitch RoomRef))

(event Custom|Show%20HUD
  (bind _self self)
  ;[1 1 1] Show HUD
  (Variables|/Script/Engine.PlayerController|SetbShowMouseCursor _self true)
  (Variables|/Script/Engine.PlayerController|SetbEnableMouseOverEvents _self true)
  (Utilities|IsValid (Variables|Default|GetHUD)
    (:Is%20Valid
      (if (UserInterface|Viewport|IsinViewport (Variables|Default|GetHUD))
        (Default|CameraSwitch (Variables|Default|GetHUD))
        (Default|F11 (Variables|Default|GetHUD) false)
        (Default|F12 (Variables|Default|GetHUD) false)
        (else
          (UserInterface|Viewport|AddtoViewport (stale _output_get) 0 :!label _label)
          (Class|PlayerController|ActivateTouchInterface (Variables|Default|GetTouch))
          (Default|F11 (Variables|Default|GetHUD) false)
          (Default|F12 (Variables|Default|GetHUD) false)
          (Default|SetPlayerName (Variables|/Game/UI/WB_HUD.WB_HUD_C|GetWB_GaugeCluster (Variables|Default|GetHUD)) (Variables|Default|GetName))
          (Default|SetEnemyName (Variables|/Game/UI/WB_HUD.WB_HUD_C|GetWB_GaugeCluster (Variables|Default|GetHUD)) (Variables|Default|GetEnemyName)))))
    (:Is%20Not%20Valid
      (Viewport|RemoveAllWidgets)
      (bind _returnvalue (UserInterface|CreateWidget "/Game/UI/WB_HUD.WB_HUD_C" self))
      (bind _output_get (Variables|Default|SetHUD _returnvalue))
      (goto _label))))

(event Custom|ClosPickUp
  (params (bNow :type Boolean))
  ;[1 1 1] PickUp HUD
  (CallFunction|PickUpAnim (Variables|Default|GetPickUpRef) false bNow))

(event Custom|Pawn%20Camera%20Setup
  (bind _hud (Variables|Default|GetHUD))
  ;[0.06667 0.06667 0.06667 0.06667] CameraTexture Switch
  (bind (_bcamera _outputpin) (Default|CameraSetup (Variables|Default|GetPlayerChar)))
  (if _bcamera
    (Class|Image|SetBrushfromMaterial (Variables|/Game/UI/WB_HUD.WB_HUD_C|GetCamera01 (Variables|Default|GetHUD)) _outputpin)
    (Default|CameraSwitch _hud 1)
    (else
      (Class|Image|SetBrushfromMaterial (Variables|/Game/UI/WB_HUD.WB_HUD_C|GetCamera02 (Variables|Default|GetHUD)) _outputpin)
      (Default|CameraSwitch _hud 1))))

(event Custom|S_EquipWeapon
  (params (Selection :type String))
  (bind _playerchar (Variables|Default|GetPlayerChar))
  ;[0.06667 0.06667 0.06667 0.06667] Melee Attack
  (Utilities|IsValid (Variables|Default|GetWeapon)
    (:Is%20Valid
      (Actor|DestroyActor (Variables|Default|GetWeapon)))
    (:Is%20Not%20Valid
      _))
  (bind _returnvalue (CallFunction|WeaponSpawn Selection))
  (bind _output_get (Variables|Default|SetWeapon _returnvalue))
  (Utilities|IsValid _playerchar
    (:Is%20Valid
      (Default|WeaponEquip _playerchar _output_get))))

(event Custom|Host
  ;[0.06667 0.06667 0.06667 0.06667] Host/Join
  (|Session self 2 false
    (:OnSuccess
      (Game|OpenLevel(byName) "Map01" true "listen"))
    (:OnFailure
      (Development|PrintString "Hosting failed!")
      (Default|StopLANHostJoin (Variables|Default|GetWBLevels)))))

(event Custom|S_SpawnDevice
  (params (Class :type Actor%20Class%20Reference) (SpawnTransform :type Transform))
  ;[0.06667 0.06667 0.06667 0.06667] Use Drop Devices
  (bind _returnvalue (Game|SpawnActorfromClass Class SpawnTransform "AlwaysSpawn" (Variables|Default|GetPlayerChar) 0))
  (Variables|Default|SetSpawnedActor _returnvalue)
  (Utilities|FlowControl|Delay 0.5)
  (Utilities|Array|Add (Variables|/Game/Blueprints/Actors/BP_Room.BP_Room_C|GetDroppedTools (Variables|/Game/Blueprints/Characters/PlayerCharacter.PlayerCharacter_C|GetRoomRef (Variables|Default|GetPlayerChar))) (Variables|Default|GetSpawnedActor)))

(event EventBeginPlay
  ;[0.06667 0.06667 0.06667 0.06667] Begin Play (SaveGameInstance, GameMode send PCtrl)
  (Networking|SwitchHasAuthority
    (:Authority
      (bind _asgm_gameplay (Utilities|Casting|CastToGM_Gameplay (Game|GetGameMode)))
      (bind _output_get (Variables|Default|SetGM _asgm_gameplay))
      (bind _returnvalue (Default|PlayersCtrls _output_get self))
      (bind _returnvalue_2 (Game|SpawnActorfromClass "/Game/Blueprints/Characters/PlayerCharacter.PlayerCharacter_C" _returnvalue "Undefined" 0 0))
      (Utilities|FlowControl|Delay 0.2)
      (CallFunction|SetUp)
      (Utilities|FlowControl|Delay 0.2)
      (Pawn|Possess _returnvalue_2))))

(event EventPossess
  (params (PossessedPawn :type Pawn%20Object%20Reference))
  ;[0.06667 0.06667 0.06667 0.06667] On Possess
  (Utilities|IsValid PossessedPawn
    (:Is%20Valid
      (bind _asplayer_character (Utilities|Casting|CastToPlayerCharacter PossessedPawn))
      (bind _output_get (Variables|Default|SetPlayerChar _asplayer_character))
      (Default|SetUPHealth _output_get)
      (Utilities|FlowControl|Delay 1.0)
      (CallFunction|ShowHUD)
      (CallFunction|PlayerCharName (Variables|Default|GetName)))))

(event Input|KeyboardEvents|Tab
  (params (Key :type Key%20Structure :default "None"))
  ;[0.06667 0.06667 0.06667 0.06667] Show Inventory
  (:Pressed
    (for _array_element (Variables|Default|GetInventory)
      (Development|PrintString (Utilities|String|Append (.itemname _array_element) (Utilities|String|ToString(Integer) (.count _array_element)))))))

(fn ConstructionScript
  (CallFunction|InventoryReset))

(fn RefreshHUD
  (Utilities|IsValid (Variables|Default|GetHUD)
    (:Is%20Valid
      (Default|CallCallHUDRefresh)
      (Default|CallCallHUDRefresh2))))

(fn OnRepBGameState
  (if (Variables|Default|GetbGameState)
    (CallFunction|GameOverUI)))

(fn InventoryConsume
  (params (ItemIndex :type Integer) (Count :type Integer))
  (bind _inventory (Variables|Default|GetInventory))
  (bind _output (Utilities|Array|Get(acopy) _inventory ItemIndex))
  (bind _returnvalue (- (.count _output) Count))
  (if (>= _returnvalue 0)
    (Utilities|Array|SetArrayElem (Variables|Default|GetInventory) ItemIndex (Utilities|Struct|MakePickUps (.itemtype _output) (.itemname _output) (.itemdescription _output) (.itemicon _output) _returnvalue (.maxcount _output) (.probability _output)))
    (return true)
    (else
      (return false))))

(fn InventoryReset
  (Utilities|Array|Clear (Variables|Default|GetInventory))
  (bind _outrownames (DataTable|GetDataTableRowNames "/Game/Data/PickupsDataTable.PickupsDataTable"))
  (for _array_element _outrownames
    (bind _returnvalue (Utilities|GetDataTableRow "/Game/Data/PickupsDataTable.PickupsDataTable" _array_element)
      (:then
        (Utilities|Array|Add (Variables|Default|GetInventory) _returnvalue))))
  (CallFunction|RefreshHUD))

(fn InventoryDrop
  (params (Selection :type String))
  (switch string Selection
    (:Laser
      (bind (_laser _transform) (|DropLaser))
      (return _laser _transform))
    (:Smoke
      (bind (_smoke _transform_2) (|Smoke))
      (return _smoke _transform_2))
    (:Trap
      (bind (_class _transform_3) (|Trap))
      (return _class _transform_3))
    (:Fire
      (bind (_class_2 _transform_4) (|Fire))
      (return _class_2 _transform_4))
    (:Mine
      (bind (_class_3 _transform_5) (|Mine))
      (return _class_3 _transform_5))
    (:Camera
      (bind (_class_4 _transform_6) (|Camera_2))
      (return _class_4 _transform_6))))

(fn ActivateAbility
  (params (bActivate :type Boolean) (AbilityName :type String))
  (bind _playerchar (Variables|Default|GetPlayerChar))
  (bind _playerchar_2 (Variables|Default|GetPlayerChar))
  (Class|KismetSystemLibrary|PauseTimer 0 "ExpendAbility")
  (if bActivate
    (bind _output_get (Variables|Default|SetActiveAbilityName AbilityName))
    (switch string _output_get
      (:Stealth
        (Variables|/Game/Blueprints/Characters/PlayerCharacter.PlayerCharacter_C|SetbStealth _playerchar_2 true))
      (:Sprint
        (Variables|/Game/Blueprints/Characters/PlayerCharacter.PlayerCharacter_C|SetMaxSpeed _playerchar_2 9e+02)))
    (Utilities|Time|SetTimerbyFunctionName 0 "ExpendAbility" 0.5 true)
    (else
      (Variables|/Game/Blueprints/Characters/PlayerCharacter.PlayerCharacter_C|SetMaxSpeed _playerchar 4e+02)
      (Variables|/Game/Blueprints/Characters/PlayerCharacter.PlayerCharacter_C|SetbStealth _playerchar false))))

(fn OnRepHealth
  (if (Pawn|IsLocalController)
    (Default|SetHealthPlayer (Variables|/Game/UI/WB_HUD.WB_HUD_C|GetWB_GaugeCluster (Variables|Default|GetHUD)) (/ (Variables|Default|GetHealth) (Variables|Default|GetMaxHealth)))
    (if (<= (Variables|Default|GetHealth) 0.0)
      (CallFunction|MatchPrep))
    (elif (<= (Variables|Default|GetHealth) 0.0)
      (Default|StADeath (Variables|Default|GetPlayerChar)))))

(fn SetEnemyName
  (params (EnemyName :type String))
  (bind _output_get (Variables|Default|SetEnemyName EnemyName))
  (Default|SetEnemyName (Variables|/Game/UI/WB_HUD.WB_HUD_C|GetWB_GaugeCluster (Variables|Default|GetHUD)) _output_get))

(fn ScoreF
  (params (Score :type Integer) (b :type Boolean)))

(fn OnRepEnemyScore
  (bind _hud (Variables|Default|GetHUD))
  (Utilities|IsValid _hud
    (:Is%20Valid
      (Default|SetEnemyScore (Variables|/Game/UI/WB_HUD.WB_HUD_C|GetWB_GaugeCluster _hud) (Variables|Default|GetEnemyScore)))))

(fn OnRepScore
  (bind _hud (Variables|Default|GetHUD))
  (Utilities|IsValid _hud
    (:Is%20Valid
      (Default|SetPlayerScore (Variables|/Game/UI/WB_HUD.WB_HUD_C|GetWB_GaugeCluster _hud) (Variables|Default|GetScore)))))

(fn WeaponSpawn
  (params (Selection :type String))
  (bind _playerchar (Variables|Default|GetPlayerChar))
  (bind _returnvalue (Transformation|GetActorTransform _playerchar))
  (switch string Selection
    (:Pistol
      (bind _returnvalue_2 (Game|SpawnActorfromClass "/Game/Blueprints/Actors/BP_Pistol.BP_Pistol_C" _returnvalue "Undefined" _playerchar 0))
      (return _returnvalue_2))
    (:Sword
      (bind _returnvalue_3 (Game|SpawnActorfromClass "/Game/Blueprints/Actors/BP_Sword.BP_Sword_C" _returnvalue "Undefined" _playerchar 0))
      (return _returnvalue_3))))

(fn CheckCount
  (params (Index :type Integer))
  (return (> (.maxcount (Utilities|Array|Get(acopy) (Variables|Default|GetInventory) Index)) 0)))

(fn EnemyHealth
  (params (Health :type Float%20%28single-precision%29))
  (Default|SetEnemyHealth (Variables|/Game/UI/WB_HUD.WB_HUD_C|GetWB_GaugeCluster (Variables|Default|GetHUD)) Health))