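; PC_MainMenu is the player controller for the main menu, handling menu screens and LAN multiplayer sessions.
; ShowMainMenu and ShowLevelList clear existing widgets, lazily create and cache their UMG widget, then show it with the cursor; only the main menu checks for local control.
; Host creates a two-connection LAN session and opens Lobby as a listen server.
; Join searches for one LAN session and joins the first result.
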(event Custom|Host
  (|Session self 2 true
    (:OnSuccess
      (Development|PrintString "Success")
      (Game|OpenLevel(byName) "Lobby" true "listen"))
    (:OnFailure
      (Development|PrintString "Hosting Failed"))))

(event Custom|Join
  (bind _results (|FindSessions self 1 true)
    (:OnSuccess
      (|JoinSession self (Utilities|Array|Get(acopy) _results)
        (:OnSuccess
          (Development|PrintString "joined success"))))
    (:OnFailure
      (Development|PrintString "Failed to join"))))

(event Custom|ShowMainMenu
  ;[1 1 1] Show Main Menu
  (if (Pawn|IsLocalController)
    (Viewport|RemoveAllWidgets)
    (Utilities|IsValid (Variables|Default|GetWBMainMenu)
      (:Is%20Valid
        _)
      (:Is%20Not%20Valid
        (bind _returnvalue (UserInterface|CreateWidget "/Game/UI/WB_MainMenu.WB_MainMenu_C" (Game|GetPlayerController 0)))
        (bind _output_get (Variables|Default|SetWBMainMenu _returnvalue))))
    (UserInterface|Viewport|AddtoViewport _output_get 0)
    (Variables|Default|SetbShowMouseCursor true)))

(event Custom|Show%20Level%20List
  ;[1 1 1] Show Level List
  (Viewport|RemoveAllWidgets)
  (Utilities|IsValid (Variables|Default|GetWBLevels)
    (:Is%20Valid
      _)
    (:Is%20Not%20Valid
      (bind _returnvalue (UserInterface|CreateWidget "/Game/UI/WB_Levels.WB_Levels_C" (Game|GetPlayerController 0)))
      (bind _output_get (Variables|Default|SetWBLevels _returnvalue))))
  (UserInterface|Viewport|AddtoViewport _output_get 0)
  (Variables|Default|SetbShowMouseCursor true))

(fn ConstructionScript)