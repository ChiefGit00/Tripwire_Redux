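; BP_Fire is a fire hazard actor that damages the player character while it overlaps the Box trigger.
; On BeginPlay it shows the Cube and holds the Box collision off for a short delay before enabling it.
; Overlap deals immediate damage and starts a looping timer that repeats the damage, spawning a bonfire sound with each hit.
; The timer clears when an overlap ends or the player's health runs out.
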(event OnComponentBeginOverlap(Box)
  (params (OverlappedComponent :type Primitive%20Component%20Object%20Reference) (OtherActor :type Actor%20Object%20Reference) (OtherComp :type Primitive%20Component%20Object%20Reference) (OtherBodyIndex :type Integer) (bFromSweep :type Boolean) (SweepResult :type Hit%20Result%20Structure%20%28by%20ref%29))
  (bind _asplayer_character (Utilities|Casting|CastToPlayerCharacter OtherActor))
  (bind _output_get (Variables|Default|SetPChar _asplayer_character))
  (Game|Damage|ApplyDamage _output_get 1e+01 0 0)
  (Audio|SpawnSoundatLocation "/Game/Audio/Bonfire_loop.Bonfire_loop" (Transformation|GetWorldLocation (Variables|Default|GetDefaultSceneRoot)) "0, 0, 0" 1.0 1.0 0.0 0 0)
  (bind _returnvalue (Utilities|Time|SetTimerbyFunctionName 0 "ApplyDamage" 0.5 true))
  (Variables|Default|SetDamageTimer _returnvalue))

(event OnComponentEndOverlap(Box)
  (params (OverlappedComponent :type Primitive%20Component%20Object%20Reference) (OtherActor :type Actor%20Object%20Reference) (OtherComp :type Primitive%20Component%20Object%20Reference) (OtherBodyIndex :type Integer))
  (Utilities|Time|ClearandInvalidateTimerbyHandle (Variables|Default|GetDamageTimer)))

(event Custom|ApplyDamage
  (if (> (Variables|/Game/Blueprints/Characters/PlayerCharacter.PlayerCharacter_C|GetHealth (Variables|Default|GetPChar)) 0.0)
    (Game|Damage|ApplyDamage (Variables|Default|GetPChar) 1e+01 0 0)
    (Audio|SpawnSoundatLocation "/Game/Audio/Bonfire_loop.Bonfire_loop" (Transformation|GetWorldLocation (Variables|Default|GetDefaultSceneRoot)) "0, 0, 0" 1.0 1.0 0.0 0 0)
    (else
      (Utilities|Time|ClearandInvalidateTimerbyHandle (Variables|Default|GetDamageTimer)))))

(event EventBeginPlay
  (Rendering|SetVisibility (Variables|Default|GetCube) true false)
  (Collision|SetCollisionEnabled (Variables|Default|GetBox) "NoCollision")
  (Utilities|FlowControl|Delay 1.0)
  (Collision|SetCollisionEnabled (Variables|Default|GetBox) "QueryAndPhysics"))

(fn ConstructionScript)