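; Thrown grenade actor that explodes on its first overlap, dealing radial damage that ignores its owning player.
; Throw launches the projectile with a given forward speed and slight lift, then after a short delay the server reports bomb use to the owner.
; Collision starts disabled and arms one second after spawn.
; Detonation also resets the owner's room smoke, plays explosion effects, hides the mesh and destroys the actor.
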(event OnComponentBeginOverlap(SphereCollision)
  (params (OverlappedComponent :type Primitive%20Component%20Object%20Reference) (OtherActor :type Actor%20Object%20Reference) (OtherComp :type Primitive%20Component%20Object%20Reference) (OtherBodyIndex :type Integer) (bFromSweep :type Boolean) (SweepResult :type Hit%20Result%20Structure%20%28by%20ref%29))
  ;[0.06667 0.06667 0.06667 0.2] On Overlap
  (Utilities|FlowControl|DoOnce false
    (:Completed
      (Game|Damage|ApplyRadialDamage 4e+01 (Transformation|GetWorldLocation (Variables|Default|GetDefaultSceneRoot)) 1e+03 0 (Variables|Default|GetActorsToAvoid) 0 0 true "ECC_Vehicle")
      (bind _asplayer_character (Utilities|Casting|CastToPlayerCharacter (Components|GetOwner)))
      (Default|ResetSmoke (Variables|/Game/Blueprints/Characters/PlayerCharacter.PlayerCharacter_C|GetRoomRef _asplayer_character))
      (Audio|PlaySoundatLocation "/Game/Audio/Bomb+2.Bomb+2" (Transformation|GetWorldLocation (Variables|Default|GetSphereCollision)) "0, 0, 0" 1.0 1.0 0.0 0 0 0)
      (Effects|Components|ParticleSystem|SetTemplate (Variables|Default|GetParticleSystem) "/Game/Particles/Fire_Exp_02.Fire_Exp_02")
      (Rendering|SetVisibility (Variables|Default|GetSphere) false false)
      (Utilities|FlowControl|Delay 0.2)
      (Actor|DestroyActor))))

(event Custom|Throw
  (params (InputPin :type Float%20%28single-precision%29))
  (bind _projectilemovement (Variables|Default|GetProjectileMovement))
  ;[0.06667 0.06667 0.06667 0.2] Throw
  (Game|Components|ProjectileMovement|SetVelocityinLocalSpace _projectilemovement (Math|Vector|MakeVector InputPin 0.0 2e+02))
  (Variables|/Script/Engine.ProjectileMovementComponent|SetbSimulationEnabled _projectilemovement true)
  (Utilities|FlowControl|Delay 1.0)
  (Networking|SwitchHasAuthority
    (:Authority
      (bind _asplayer_character (Utilities|Casting|CastToPlayerCharacter (Components|GetOwner)))
      (Default|OCWeaponUsed _asplayer_character "Bomb"))))

(event EventBeginPlay
  ;[0.06667 0.06667 0.06667 0.2] BeginPlay
  (Utilities|Array|Add (Variables|Default|GetActorsToAvoid) (Components|GetOwner))
  (Utilities|FlowControl|Delay 1.0)
  (Collision|SetCollisionEnabled (Variables|Default|GetSphereCollision) "QueryAndPhysics"))

(fn ConstructionScript
  (Collision|SetCollisionEnabled (Variables|Default|GetSphereCollision) "NoCollision"))