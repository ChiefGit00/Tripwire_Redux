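; BP_PickUp is a clickable or tappable loot container that opens and closes with animation, sound and material changes.
; A box overlap grants the player access, highlights the switch material and toggles a one-time help hint.
; When ready, a press suppresses jumping, asks PC_Gameplay to animate it, then rolls each pickups DataTable row by probability for the HUD.
; Leaving hides that HUD, and closing re-arms the pickup after a delay.
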(event OnComponentBeginOverlap(Box)
  (params (OverlappedComponent :type Primitive%20Component%20Object%20Reference) (OtherActor :type Actor%20Object%20Reference) (OtherComp :type Primitive%20Component%20Object%20Reference) (OtherBodyIndex :type Integer) (bFromSweep :type Boolean) (SweepResult :type Hit%20Result%20Structure%20%28by%20ref%29))
  ;[0.06667 0.06667 0.06667 0.2 16] Pickup Activation
  (Utilities|Casting|CastToPlayerCharacter OtherActor)
  (Rendering|Material|SetMaterial (Variables|Default|GetSkeletalMesh) 1 "/Game/Materials/M_SwitchActive.M_SwitchActive")
  (Variables|Default|SetbAccess true)
  (if (Variables|Default|GetbHelper)
    (Rendering|SetVisibility (Variables|Default|GetHelp) true false)))

(event OnComponentEndOverlap(Box)
  (params (OverlappedComponent :type Primitive%20Component%20Object%20Reference) (OtherActor :type Actor%20Object%20Reference) (OtherComp :type Primitive%20Component%20Object%20Reference) (OtherBodyIndex :type Integer))
  ;[0.06667 0.06667 0.06667 0.2 16] Pickup Activation
  (Utilities|Casting|CastToPlayerCharacter OtherActor)
  (Rendering|Material|SetMaterial (Variables|Default|GetSkeletalMesh) 1 "/Game/Materials/M_SwitchDeactive1.M_SwitchDeactive1")
  (Variables|Default|SetbAccess false)
  (if (Variables|Default|GetbOpen)
    (Default|HUDPickUPHide (Variables|Default|GetPC) true))
  (if (Variables|Default|GetbHelper)
    (Rendering|SetVisibility (Variables|Default|GetHelp) false false)))

(event Custom|PlayOpenAnimation
  (params (bOpen :type Boolean) (Duration :type Float%20%28single-precision%29))
  (bind _skeletalmesh (Variables|Default|GetSkeletalMesh))
  ;[0.06667 0.06667 0.06667 0.2] Open/Close animation
  (if bOpen
    (Components|Animation|PlayAnimation _skeletalmesh "/Game/SkeletalMeshes/pickupOpen_Anim.pickupOpen_Anim" false)
    (Audio|PlaySoundatLocation "/Game/Audio/CameraClose.CameraClose" (Transformation|GetWorldLocation (Variables|Default|GetSkeletalMesh)) "0, 0, 0" 1.0 1.0 0.0 0 0 0)
    (Variables|Default|SetbOpen true)
    (Variables|Default|SetbReady false)
    (Rendering|Material|SetMaterial (Variables|Default|GetSkeletalMesh) 0 "/Game/Materials/CubeMaterial.CubeMaterial")
    (else
      (Components|Animation|PlayAnimation _skeletalmesh "/Game/SkeletalMeshes/pickupClose.pickupClose" false)
      (Audio|PlaySoundatLocation "/Game/Audio/DrawerClose.DrawerClose" (Transformation|GetWorldLocation (Variables|Default|GetSkeletalMesh)) "0, 0, 0" 1.0 1.0 0.0 0 0 0)
      (Variables|Default|SetbOpen false)
      (Utilities|FlowControl|Delay Duration)
      (Variables|Default|SetbReady true)
      (Rendering|Material|SetMaterial (Variables|Default|GetSkeletalMesh) 0 "/Game/Materials/Center.Center"))))

(event EventActorOnInputTouchBegin
  (params (FingerIndex :type ETouchIndex%20Enum :default "Touch1"))
  ;[0.06667 0.06667 0.06667 0.2 16] OnClicked
  (if (Variables|Default|GetbAccess)
    (bind _asplayer_character (Utilities|Casting|CastToPlayerCharacter (Game|Player|GetPlayerPawn 0)))
    (bind _output_get (Variables|Default|SetPChar _asplayer_character))
    (Variables|/Game/Blueprints/Characters/PlayerCharacter.PlayerCharacter_C|SetbJump _output_get false)
    (if (Variables|Default|GetbReady)
      (if (Variables|Default|GetbHelper)
        (Rendering|SetVisibility (Variables|Default|GetHelp) false false)
        (Variables|Default|SetbHelper false))
      (bind _aspc_gameplay (Utilities|Casting|CastToPC_Gameplay (Game|GetPlayerController 0)))
      (bind _output_get_2 (Variables|Default|SetPC _aspc_gameplay))
      (Default|PickUpAnim _output_get_2 self true false)
      (Utilities|Array|Clear (Variables|Default|GetPickUpCount))
      (bind _outrownames (DataTable|GetDataTableRowNames "/Game/Data/PickupsDataTable.PickupsDataTable"))
      (for _array_element _outrownames
        (bind _returnvalue (Utilities|GetDataTableRow "/Game/Data/PickupsDataTable.PickupsDataTable" _array_element)
          (:then
            (if (Math|Random|RandomBoolwithWeight (.probability _returnvalue))
              (Utilities|Array|Add (Variables|Default|GetPickUpCount) (Utilities|Struct|MakePickUpsCounts (.itemname _returnvalue) 1 (.itemtype _returnvalue)))))))
      (Default|HUDPickUPShow (Variables|Default|GetPC) (Variables|Default|GetPickUpCount)))))

(event MouseInput|EventActorOnClicked
  (params (ButtonPressed :type Key%20Structure :default "None"))
  ;[0.06667 0.06667 0.06667 0.2 16] OnClicked
  (if (Variables|Default|GetbAccess)
    (bind _asplayer_character (Utilities|Casting|CastToPlayerCharacter (Game|Player|GetPlayerPawn 0)))
    (bind _output_get (Variables|Default|SetPChar _asplayer_character))
    (Variables|/Game/Blueprints/Characters/PlayerCharacter.PlayerCharacter_C|SetbJump _output_get false)
    (if (Variables|Default|GetbReady)
      (if (Variables|Default|GetbHelper)
        (Rendering|SetVisibility (Variables|Default|GetHelp) false false)
        (Variables|Default|SetbHelper false))
      (bind _aspc_gameplay (Utilities|Casting|CastToPC_Gameplay (Game|GetPlayerController 0)))
      (bind _output_get_2 (Variables|Default|SetPC _aspc_gameplay))
      (Default|PickUpAnim _output_get_2 self true false)
      (Utilities|Array|Clear (Variables|Default|GetPickUpCount))
      (bind _outrownames (DataTable|GetDataTableRowNames "/Game/Data/PickupsDataTable.PickupsDataTable"))
      (for _array_element _outrownames
        (bind _returnvalue (Utilities|GetDataTableRow "/Game/Data/PickupsDataTable.PickupsDataTable" _array_element)
          (:then
            (if (Math|Random|RandomBoolwithWeight (.probability _returnvalue))
              (Utilities|Array|Add (Variables|Default|GetPickUpCount) (Utilities|Struct|MakePickUpsCounts (.itemname _returnvalue) 1 (.itemtype _returnvalue)))))))
      (Default|HUDPickUPShow (Variables|Default|GetPC) (Variables|Default|GetPickUpCount)))))

(event EventActorOnInputTouchEnd
  (params (FingerIndex :type ETouchIndex%20Enum :default "Touch1"))
  (bind _pchar (Variables|Default|GetPChar))
  ;[0.06667 0.06667 0.06667 0.2] Open/Close animation
  (Utilities|IsValid _pchar
    (:Is%20Valid
      (Variables|/Game/Blueprints/Characters/PlayerCharacter.PlayerCharacter_C|SetbJump _pchar true))))

(event EventActorOnReleased
  (params (ButtonReleased :type Key%20Structure :default "None"))
  (bind _pchar (Variables|Default|GetPChar))
  ;[0.06667 0.06667 0.06667 0.2] Open/Close animation
  (Utilities|IsValid _pchar
    (:Is%20Valid
      (Variables|/Game/Blueprints/Characters/PlayerCharacter.PlayerCharacter_C|SetbJump _pchar true))))

(fn ConstructionScript
  (bind _returnvalue (Rendering|Material|CreateDynamicMaterialInstance (Variables|Default|GetSkeletalMesh) 1 0 "None" :!class /Script/Engine.PrimitiveComponent))
  (Variables|Default|SetBorderMI _returnvalue))

(fn OnRepBOpen
  (Components|Animation|PlayAnimation (Variables|Default|GetSkeletalMesh) "/Game/SkeletalMeshes/pickupOpen_Anim.pickupOpen_Anim" false))

(fn Size
  (Transformation|SetWorldScale3D (Variables|Default|GetSkeletalMesh) "2.000000,2.000000,0.000000"))