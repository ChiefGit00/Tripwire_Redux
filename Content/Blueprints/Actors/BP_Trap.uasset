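; Trap actor that freezes any PlayerCharacter stepping into its box by disabling their input for two seconds.
; Box collision arms one second after BeginPlay to query-only.
; When triggered, the cube drops owner-only visibility, switches to the deactivated material and plays a sound, then restores both visibility and material along with input.
; ShowAll, ShowOwnerOnly and HideAll events let the cube's visibility be set directly.
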(event OnComponentBeginOverlap(Box)
  (params (OverlappedComponent :type Primitive%20Component%20Object%20Reference) (OtherActor :type Actor%20Object%20Reference) (OtherComp :type Primitive%20Component%20Object%20Reference) (OtherBodyIndex :type Integer) (bFromSweep :type Boolean) (SweepResult :type Hit%20Result%20Structure%20%28by%20ref%29))
  (bind _asplayer_character (Utilities|Casting|CastToPlayerCharacter OtherActor))
  (Input|DisableInput _asplayer_character 0)
  (Rendering|SetOnlyOwnerSee (Variables|Default|GetCube) false :!class /Script/Engine.PrimitiveComponent)
  (Rendering|Material|SetMaterial (Variables|Default|GetCube) 0 "/Game/Materials/M_SwitchDeactive.M_SwitchDeactive")
  (Audio|PlaySoundatLocation "/Game/Audio/Trap.Trap" (Transformation|GetActorLocation) "0, 0, 0" 1.0 1.0 0.0 0 0 0)
  (Utilities|FlowControl|Delay 2.0)
  (Input|EnableInput _asplayer_character 0)
  (Rendering|SetOnlyOwnerSee (Variables|Default|GetCube) true :!class /Script/Engine.PrimitiveComponent)
  (Rendering|Material|SetMaterial (Variables|Default|GetCube) 0 "/Game/Materials/M_SwitchActive_Inst1.M_SwitchActive_Inst1"))

(event EventShowAll
  (bind _cube (Variables|Default|GetCube))
  (Rendering|SetVisibility _cube true false)
  (Rendering|SetOnlyOwnerSee _cube false :!class /Script/Engine.PrimitiveComponent))

(event EventShowOwnerOnly
  (bind _cube (Variables|Default|GetCube))
  (Rendering|SetVisibility _cube true false)
  (Rendering|SetOnlyOwnerSee _cube true :!class /Script/Engine.PrimitiveComponent))

(event EventHideAll
  (Rendering|SetVisibility (Variables|Default|GetCube) false false))

(event EventBeginPlay
  (Collision|SetCollisionEnabled (Variables|Default|GetBox) "NoCollision")
  (Utilities|FlowControl|Delay 1.0)
  (Collision|SetCollisionEnabled (Variables|Default|GetBox) "QueryOnly"))

(fn ConstructionScript)