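; BP_Sword is a melee weapon actor that damages player characters other than its owner.
; SwordAttack plays a swoosh and briefly enables query collision on the capsule, which is otherwise disabled from BeginPlay.
; An overlap with another player applies fixed damage, then toggles mesh visibility after a short delay.
; After a second delay, the authority notifies the owning character through OCWeaponUsed that the sword was used.
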(event OnComponentBeginOverlap(Capsule)
  (params (OverlappedComponent :type Primitive%20Component%20Object%20Reference) (OtherActor :type Actor%20Object%20Reference) (OtherComp :type Primitive%20Component%20Object%20Reference) (OtherBodyIndex :type Integer) (bFromSweep :type Boolean) (SweepResult :type Hit%20Result%20Structure%20%28by%20ref%29))
  (bind _asplayer_character (Utilities|Casting|CastToPlayerCharacter OtherActor))
  (if (not (== _asplayer_character (Components|GetOwner)))
    (Game|Damage|ApplyDamage _asplayer_character 3e+01 0 0)
    (Utilities|FlowControl|Delay 0.4)
    (Rendering|ToggleVisibility (Variables|Default|GetSkeletalMesh) false)
    (Utilities|FlowControl|Delay 0.4)
    (Networking|SwitchHasAuthority
      (:Authority
        (bind _asplayer_character_2 (Utilities|Casting|CastToPlayerCharacter (Components|GetOwner)))
        (Default|OCWeaponUsed _asplayer_character_2 "Sword")))))

(event Custom|SwordAttack
  (bind _capsule (Variables|Default|GetCapsule))
  (Collision|SetCollisionEnabled _capsule "QueryOnly")
  (Audio|PlaySoundatLocation "/Game/Audio/SwordSwoosh.SwordSwoosh" (Transformation|GetWorldLocation (Variables|Default|GetDefaultSceneRoot)) "0, 0, 0" 1.0 1.0 0.0 0 0 0)
  (Utilities|FlowControl|Delay 0.4)
  (Collision|SetCollisionEnabled _capsule "NoCollision"))

(event EventBeginPlay
  (Collision|SetCollisionEnabled (Variables|Default|GetCapsule) "NoCollision"))

(fn ConstructionScript)