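; Lobby game mode that gathers joining players and moves the match to Map01 once more than one is present.
; On PostLogin it stores and initializes each PC_Lobby controller and increments the player count.
; With enough players, it waits briefly, then passes every controller the other players' names and match records.
; It then starts the countdown on all controllers and runs a servertravel console command after a delay.
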(event EventPostLogin
  (params (NewPlayer :type Player%20Controller%20Object%20Reference))
  (bind _playerctrls (Variables|Default|GetPlayerCtrls))
  (bind _aspc_lobby (Utilities|Casting|CastToPC_Lobby NewPlayer))
  (Utilities|Array|Add (Variables|Default|GetPlayerCtrls) _aspc_lobby)
  (Default|Initialize _aspc_lobby)
  (bind _result (Math|Integer|IncrementInt (Variables|Default|GetPlayerCount))
    (:%20%20
      (if (> _result 1)
        (Utilities|FlowControl|Delay 1.0)
        (for _array_element _playerctrls
          (for _array_element_2 _playerctrls
            (if (not (== _array_element_2 _array_element))
              (Default|SetUpPlayer _array_element false (Variables|/Game/Blueprints/Gameplay/PC_Lobby.PC_Lobby_C|GetPlayerName _array_element_2) (Variables|/Game/Blueprints/Gameplay/PC_Lobby.PC_Lobby_C|GetGamesPlayed _array_element_2) (Variables|/Game/Blueprints/Gameplay/PC_Lobby.PC_Lobby_C|GetGamesWon _array_element_2) (Variables|/Game/Blueprints/Gameplay/PC_Lobby.PC_Lobby_C|GetGamesLost _array_element_2)))))
        (for _array_element_3 (Variables|Default|GetPlayerCtrls)
          (Default|StartCountdown _array_element_3))
        (Utilities|FlowControl|Delay 3.0)
        (Development|ExecuteConsoleCommand "servertravel Map01" 0)))))

(fn ConstructionScript)