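; BP_StairsUp is a staircase actor that remaps PlayerCharacter movement axes as the player climbs or descends it.
; A series of trigger boxes toggles the character's Xaxis, Yaxis, SwapAxis and YaxisFlip flags on overlap.
; Box3 and Box4 latch Up or Down by entry order, letting shared triggers act according to travel direction.
; Several end boxes switch Yaxis off and clear the direction state.
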(event OnComponentBeginOverlap(Collision8)
  (params (OverlappedComponent :type Primitive%20Component%20Object%20Reference) (OtherActor :type Actor%20Object%20Reference) (OtherComp :type Primitive%20Component%20Object%20Reference) (OtherBodyIndex :type Integer) (bFromSweep :type Boolean) (SweepResult :type Hit%20Result%20Structure%20%28by%20ref%29))
  ;[1 1 1 0 16] Box
  (bind _asplayer_character (Utilities|Casting|CastToPlayerCharacter OtherActor))
  (Variables|/Game/Blueprints/Characters/PlayerCharacter.PlayerCharacter_C|SetbYaxis _asplayer_character true))

(event OnComponentBeginOverlap(Box1)
  (params (OverlappedComponent :type Primitive%20Component%20Object%20Reference) (OtherActor :type Actor%20Object%20Reference) (OtherComp :type Primitive%20Component%20Object%20Reference) (OtherBodyIndex :type Integer) (bFromSweep :type Boolean) (SweepResult :type Hit%20Result%20Structure%20%28by%20ref%29))
  ;[1 1 1 0 16] Box 1
  (bind _asplayer_character (Utilities|Casting|CastToPlayerCharacter OtherActor))
  (Variables|/Game/Blueprints/Characters/PlayerCharacter.PlayerCharacter_C|SetbSwapAxis _asplayer_character true))

(event OnComponentBeginOverlap(Box9)
  (params (OverlappedComponent :type Primitive%20Component%20Object%20Reference) (OtherActor :type Actor%20Object%20Reference) (OtherComp :type Primitive%20Component%20Object%20Reference) (OtherBodyIndex :type Integer) (bFromSweep :type Boolean) (SweepResult :type Hit%20Result%20Structure%20%28by%20ref%29))
  ;[1 1 1 0 16] Box 9
  (bind _asplayer_character (Utilities|Casting|CastToPlayerCharacter OtherActor))
  (if (Variables|/Game/Blueprints/Characters/PlayerCharacter.PlayerCharacter_C|GetbDown _asplayer_character)
    (Variables|/Game/Blueprints/Characters/PlayerCharacter.PlayerCharacter_C|SetbSwapAxis _asplayer_character false)
    (Variables|/Game/Blueprints/Characters/PlayerCharacter.PlayerCharacter_C|SetbYaxisFlip _asplayer_character true)))

(event OnComponentBeginOverlap(Box6)
  (params (OverlappedComponent :type Primitive%20Component%20Object%20Reference) (OtherActor :type Actor%20Object%20Reference) (OtherComp :type Primitive%20Component%20Object%20Reference) (OtherBodyIndex :type Integer) (bFromSweep :type Boolean) (SweepResult :type Hit%20Result%20Structure%20%28by%20ref%29))
  ;[1 1 1 0 16] End Yaxis
  (bind _asplayer_character (Utilities|Casting|CastToPlayerCharacter OtherActor))
  (Variables|/Game/Blueprints/Characters/PlayerCharacter.PlayerCharacter_C|SetbYaxis _asplayer_character false)
  (Variables|/Game/Blueprints/Characters/PlayerCharacter.PlayerCharacter_C|SetbUp _asplayer_character false)
  (Variables|/Game/Blueprints/Characters/PlayerCharacter.PlayerCharacter_C|SetbDown _asplayer_character false))

(event OnComponentEndOverlap(Box3)
  (params (OverlappedComponent :type Primitive%20Component%20Object%20Reference) (OtherActor :type Actor%20Object%20Reference) (OtherComp :type Primitive%20Component%20Object%20Reference) (OtherBodyIndex :type Integer))
  ;[1 1 1 0 16] Box 3
  (bind _asplayer_character (Utilities|Casting|CastToPlayerCharacter OtherActor))
  (if (Variables|/Game/Blueprints/Characters/PlayerCharacter.PlayerCharacter_C|GetbDown _asplayer_character)
    (Variables|/Game/Blueprints/Characters/PlayerCharacter.PlayerCharacter_C|SetbDown _asplayer_character false)
    (Variables|/Game/Blueprints/Characters/PlayerCharacter.PlayerCharacter_C|SetbYaxisFlip _asplayer_character false)
    (Variables|/Game/Blueprints/Characters/PlayerCharacter.PlayerCharacter_C|SetbXaxis _asplayer_character true)
    (elif (Variables|/Game/Blueprints/Characters/PlayerCharacter.PlayerCharacter_C|GetbUp _asplayer_character)
      (Variables|/Game/Blueprints/Characters/PlayerCharacter.PlayerCharacter_C|SetbXaxis _asplayer_character false))))

(event OnComponentBeginOverlap(Box8)
  (params (OverlappedComponent :type Primitive%20Component%20Object%20Reference) (OtherActor :type Actor%20Object%20Reference) (OtherComp :type Primitive%20Component%20Object%20Reference) (OtherBodyIndex :type Integer) (bFromSweep :type Boolean) (SweepResult :type Hit%20Result%20Structure%20%28by%20ref%29))
  ;[1 1 1 0 16] End Yaxis
  (bind _asplayer_character (Utilities|Casting|CastToPlayerCharacter OtherActor))
  (Variables|/Game/Blueprints/Characters/PlayerCharacter.PlayerCharacter_C|SetbYaxis _asplayer_character false)
  (Variables|/Game/Blueprints/Characters/PlayerCharacter.PlayerCharacter_C|SetbUp _asplayer_character false)
  (Variables|/Game/Blueprints/Characters/PlayerCharacter.PlayerCharacter_C|SetbDown _asplayer_character false))

(event OnComponentBeginOverlap(Box7)
  (params (OverlappedComponent :type Primitive%20Component%20Object%20Reference) (OtherActor :type Actor%20Object%20Reference) (OtherComp :type Primitive%20Component%20Object%20Reference) (OtherBodyIndex :type Integer) (bFromSweep :type Boolean) (SweepResult :type Hit%20Result%20Structure%20%28by%20ref%29))
  ;[1 1 1 0 16] End Yaxis
  (bind _asplayer_character (Utilities|Casting|CastToPlayerCharacter OtherActor))
  (Variables|/Game/Blueprints/Characters/PlayerCharacter.PlayerCharacter_C|SetbYaxis _asplayer_character false)
  (Variables|/Game/Blueprints/Characters/PlayerCharacter.PlayerCharacter_C|SetbUp _asplayer_character false)
  (Variables|/Game/Blueprints/Characters/PlayerCharacter.PlayerCharacter_C|SetbDown _asplayer_character false))

(event OnComponentEndOverlap(Box1)
  (params (OverlappedComponent :type Primitive%20Component%20Object%20Reference) (OtherActor :type Actor%20Object%20Reference) (OtherComp :type Primitive%20Component%20Object%20Reference) (OtherBodyIndex :type Integer))
  ;[1 1 1 0 16] Box 1
  (bind _asplayer_character (Utilities|Casting|CastToPlayerCharacter OtherActor))
  (if (not (Variables|/Game/Blueprints/Characters/PlayerCharacter.PlayerCharacter_C|GetbDown _asplayer_character))
    (Variables|/Game/Blueprints/Characters/PlayerCharacter.PlayerCharacter_C|SetbSwapAxis _asplayer_character false)
    (Variables|/Game/Blueprints/Characters/PlayerCharacter.PlayerCharacter_C|SetbYaxisFlip _asplayer_character true)))

(event OnComponentBeginOverlap(Box2)
  (params (OverlappedComponent :type Primitive%20Component%20Object%20Reference) (OtherActor :type Actor%20Object%20Reference) (OtherComp :type Primitive%20Component%20Object%20Reference) (OtherBodyIndex :type Integer) (bFromSweep :type Boolean) (SweepResult :type Hit%20Result%20Structure%20%28by%20ref%29))
  ;[1 1 1 0 16] Box 2
  (bind _asplayer_character (Utilities|Casting|CastToPlayerCharacter OtherActor))
  (Variables|/Game/Blueprints/Characters/PlayerCharacter.PlayerCharacter_C|SetbYaxis _asplayer_character true)
  (Variables|/Game/Blueprints/Characters/PlayerCharacter.PlayerCharacter_C|SetbXaxis _asplayer_character true)
  (Variables|/Game/Blueprints/Characters/PlayerCharacter.PlayerCharacter_C|SetbSwapAxis _asplayer_character false))

(event OnComponentBeginOverlap(Box5)
  (params (OverlappedComponent :type Primitive%20Component%20Object%20Reference) (OtherActor :type Actor%20Object%20Reference) (OtherComp :type Primitive%20Component%20Object%20Reference) (OtherBodyIndex :type Integer) (bFromSweep :type Boolean) (SweepResult :type Hit%20Result%20Structure%20%28by%20ref%29))
  ;[1 1 1 0 16] End Yaxis
  (bind _asplayer_character (Utilities|Casting|CastToPlayerCharacter OtherActor))
  (Variables|/Game/Blueprints/Characters/PlayerCharacter.PlayerCharacter_C|SetbYaxis _asplayer_character false)
  (Variables|/Game/Blueprints/Characters/PlayerCharacter.PlayerCharacter_C|SetbUp _asplayer_character false)
  (Variables|/Game/Blueprints/Characters/PlayerCharacter.PlayerCharacter_C|SetbDown _asplayer_character false))

(event OnComponentBeginOverlap(Box3)
  (params (OverlappedComponent :type Primitive%20Component%20Object%20Reference) (OtherActor :type Actor%20Object%20Reference) (OtherComp :type Primitive%20Component%20Object%20Reference) (OtherBodyIndex :type Integer) (bFromSweep :type Boolean) (SweepResult :type Hit%20Result%20Structure%20%28by%20ref%29))
  ;[1 1 1 0 16] Box 3
  (bind _asplayer_character (Utilities|Casting|CastToPlayerCharacter OtherActor))
  (if (not (Variables|/Game/Blueprints/Characters/PlayerCharacter.PlayerCharacter_C|GetbDown _asplayer_character))
    (Variables|/Game/Blueprints/Characters/PlayerCharacter.PlayerCharacter_C|SetbUp _asplayer_character true)))

(event OnComponentEndOverlap(Box4)
  (params (OverlappedComponent :type Primitive%20Component%20Object%20Reference) (OtherActor :type Actor%20Object%20Reference) (OtherComp :type Primitive%20Component%20Object%20Reference) (OtherBodyIndex :type Integer))
  ;[1 1 1 0 16] Box 4 (Top Stair Entry)
  (bind _asplayer_character (Utilities|Casting|CastToPlayerCharacter OtherActor))
  (if (Variables|/Game/Blueprints/Characters/PlayerCharacter.PlayerCharacter_C|GetbUp _asplayer_character)
    (Variables|/Game/Blueprints/Characters/PlayerCharacter.PlayerCharacter_C|SetbXaxis _asplayer_character true)
    (Variables|/Game/Blueprints/Characters/PlayerCharacter.PlayerCharacter_C|SetbYaxisFlip _asplayer_character false)
    (Variables|/Game/Blueprints/Characters/PlayerCharacter.PlayerCharacter_C|SetbUp _asplayer_character false)
    (elif (Variables|/Game/Blueprints/Characters/PlayerCharacter.PlayerCharacter_C|GetbDown _asplayer_character)
      (Variables|/Game/Blueprints/Characters/PlayerCharacter.PlayerCharacter_C|SetbXaxis _asplayer_character false))))

(event OnComponentBeginOverlap(Box4)
  (params (OverlappedComponent :type Primitive%20Component%20Object%20Reference) (OtherActor :type Actor%20Object%20Reference) (OtherComp :type Primitive%20Component%20Object%20Reference) (OtherBodyIndex :type Integer) (bFromSweep :type Boolean) (SweepResult :type Hit%20Result%20Structure%20%28by%20ref%29))
  ;[1 1 1 0 16] Box 4 (Top Stair Entry)
  (bind _asplayer_character (Utilities|Casting|CastToPlayerCharacter OtherActor))
  (if (not (Variables|/Game/Blueprints/Characters/PlayerCharacter.PlayerCharacter_C|GetbUp _asplayer_character))
    (Variables|/Game/Blueprints/Characters/PlayerCharacter.PlayerCharacter_C|SetbDown _asplayer_character true)))

(event OnComponentBeginOverlap(Box10)
  (params (OverlappedComponent :type Primitive%20Component%20Object%20Reference) (OtherActor :type Actor%20Object%20Reference) (OtherComp :type Primitive%20Component%20Object%20Reference) (OtherBodyIndex :type Integer) (bFromSweep :type Boolean) (SweepResult :type Hit%20Result%20Structure%20%28by%20ref%29))
  ;[1 1 1 0 16] Box 10
  (bind _asplayer_character (Utilities|Casting|CastToPlayerCharacter OtherActor))
  (if (Variables|/Game/Blueprints/Characters/PlayerCharacter.PlayerCharacter_C|GetbDown _asplayer_character)
    (Variables|/Game/Blueprints/Characters/PlayerCharacter.PlayerCharacter_C|SetbSwapAxis _asplayer_character true)))

(fn ConstructionScript)